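; Health component that tracks an owner's current health and dead state, starting at max health on BeginPlay.
; GainHealth and TakeHealth adjust health clamped between zero and max and return the new value, with HealthUpdate wrapping TakeHealth.
; When TakeHealth finds no health left, Death sets the Dead flag and calls OnDeath, guarded by a DoOnce.
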(event EventBeginPlay
  (Variables|Default|SetDead false)
  (Variables|Default|SetCurrentHealth (Variables|Default|GetMaxHealth)))

(fn GainHealth
  (params (Health :type Float%20%28double-precision%29))
  (bind _output_get (Variables|Default|SetCurrentHealth (Math|Float|Clamp(Float) (+ Health (Variables|Default|GetCurrentHealth)) 0.0 (Variables|Default|GetMaxHealth))))
  (return _output_get))

(fn TakeHealth
  (params (Damage :type Float%20%28double-precision%29))
  (Variables|Default|SetCurrentHealth (Math|Float|Clamp(Float) (- (Variables|Default|GetCurrentHealth) Damage) 0.0 (Variables|Default|GetMaxHealth)))
  (if (Utilities|HasHealth)
    _
    (else
      (CallFunction|Death)))
  (return (Variables|Default|GetCurrentHealth)))

(fn Death
  (Utilities|FlowControl|DoOnce false
    (:Completed
      (Variables|Default|SetDead true)
      (Default|CallOnDeath))))

(fn HealthUpdate
  (params (Damage :type Float%20%28double-precision%29))
  (bind _currenthealth (CallFunction|TakeHealth Damage))
  (return _currenthealth))