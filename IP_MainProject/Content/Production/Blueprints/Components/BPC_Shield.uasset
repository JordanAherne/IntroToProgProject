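; Actor component that gives its owner a shield state with a matching visual.
; On BeginPlay it spawns a BP_Shield actor, attaches it to the owner and hides its Shield component.
; AddShield and RemoveShield set the HasShield flag and show or hide that component to match, reusing the one spawned actor.
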(event Custom|RemoveShield
  (bind _output_get (Variables|Default|SethasShield false))
  (Rendering|SetVisibility (Variables|/Game/Production/Blueprints/LevelComponents/BP_Shield.BP_Shield_C|GetShield (Variables|Default|GetShieldBP)) _output_get false))

(event Custom|AddShield
  (bind _output_get (Variables|Default|SethasShield true))
  (Rendering|SetVisibility (Variables|/Game/Production/Blueprints/LevelComponents/BP_Shield.BP_Shield_C|GetShield (Variables|Default|GetShieldBP)) _output_get false))

(event EventBeginPlay
  (bind _returnvalue (Game|SpawnActorfromClass "/Game/Production/Blueprints/LevelComponents/BP_Shield.BP_Shield_C" (Math|Transform|MakeTransform "0, 0, 0" "0, 0, 0" "1.000000,1.000000,1.000000") "Undefined" "MultiplyWithRoot" 0 0))
  (bind _output_get (Variables|Default|SetShieldBP _returnvalue))
  (Transformation|AttachActorToActor _output_get (Components|GetOwner self) "None" "KeepRelative" "KeepRelative" "KeepRelative" true)
  (Rendering|SetVisibility (Variables|/Game/Production/Blueprints/LevelComponents/BP_Shield.BP_Shield_C|GetShield (Variables|Default|GetShieldBP)) false false))