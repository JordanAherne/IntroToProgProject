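; Floating component that moves a referenced component up and down between top and bottom relative positions.
; While Enabled, Tick passes through a DoOnce into two chained MoveComponentTo moves, to TopPos then BottomPos, with configurable easing and duration.
; The final move wires back to the Enabled check, but no DoOnce reset is shown, so the graph as written runs only one cycle.
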(event EventBeginPlay)

(event EventTick
  (params (DeltaSeconds :type Float%20%28single-precision%29))
  (if (Variables|Default|Getenabled) :!label _label
    (Utilities|FlowControl|DoOnce false
      (:Completed
        (Components|MoveComponentTo (Variables|Default|GetComponent) (Variables|Default|GetTopPos) "0, 0, 0" (Variables|Default|GetEase%20Out) (Variables|Default|GetEase%20In) (Variables|Default|GetOver%20Time) false)
        (Components|MoveComponentTo (Variables|Default|GetComponent) (Variables|Default|GetBottomPos) "0, 0, 0" (Variables|Default|GetEase%20Out) (Variables|Default|GetEase%20In) (Variables|Default|GetOver%20Time) false)
        (goto _label)))))