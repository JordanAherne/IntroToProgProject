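; Ammo inventory component that tracks separate reserves for Light, Medium, Heavy, Shotgun and Energy ammo types.
; BeginPlay fills Light, Medium and Shotgun to their maximums, sets Heavy from the Medium maximum, and leaves Energy at its default.
; AddAmmo and RemoveAmmo switch on ammo type and clamp the count between zero and that type's maximum.
; GetAmmoOfType returns the count and whether any remains, while IsFull compares it to the maximum.
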(event EventBeginPlay
  (Variables|Default|SetLight%20Ammo (Variables|Default|GetMax%20Light%20Ammo))
  (Variables|Default|SetMedium%20Ammo (Variables|Default|GetMax%20Medium%20Ammo))
  (Variables|Default|SetHeavy%20Ammo (Variables|Default|GetMax%20Medium%20Ammo))
  (Variables|Default|SetShotgun%20Ammo (Variables|Default|GetMax%20Shotgun%20Ammo)))

(event EventTick
  (params (DeltaSeconds :type Float%20%28single-precision%29)))

(fn AddAmmo
  (params (AmmoAmount :type Integer) (AmmoType :type Enum_AmmoType%20Enum :default "NewEnumerator0"))
  (Variables|Default|SetAmmoToAdd AmmoAmount)
  (switch Utilities|FlowControl|Switch|SwitchonEnum_AmmoType AmmoType
    (:NewEnumerator0
      (Variables|Default|SetLight%20Ammo (Math|Integer|Clamp(Integer) (+ (Variables|Default|GetLight%20Ammo) (Variables|Default|GetAmmoToAdd)) 0 (Variables|Default|GetMax%20Light%20Ammo))))
    (:NewEnumerator1
      (Variables|Default|SetMedium%20Ammo (Math|Integer|Clamp(Integer) (+ (Variables|Default|GetMedium%20Ammo) (Variables|Default|GetAmmoToAdd)) 0 (Variables|Default|GetMax%20Medium%20Ammo))))
    (:NewEnumerator2
      (Variables|Default|SetHeavy%20Ammo (Math|Integer|Clamp(Integer) (+ (Variables|Default|GetHeavy%20Ammo) (Variables|Default|GetAmmoToAdd)) 0 (Variables|Default|GetMax%20Heavy%20Ammo))))
    (:NewEnumerator3
      (Variables|Default|SetShotgun%20Ammo (Math|Integer|Clamp(Integer) (+ (Variables|Default|GetShotgun%20Ammo) (Variables|Default|GetAmmoToAdd)) 0 (Variables|Default|GetMax%20Shotgun%20Ammo))))
    (:NewEnumerator4
      (Variables|Default|SetEnergy%20Ammo (Math|Integer|Clamp(Integer) (+ (Variables|Default|GetEnergy%20Ammo) (Variables|Default|GetAmmoToAdd)) 0 (Variables|Default|GetMax%20Energy%20Ammo))))))

(fn RemoveAmmo
  (params (AmmoAmount :type Integer) (AmmoType :type Enum_AmmoType%20Enum :default "NewEnumerator0"))
  (Variables|Default|SetAmmoToRemove AmmoAmount)
  (switch Utilities|FlowControl|Switch|SwitchonEnum_AmmoType AmmoType
    (:NewEnumerator0
      (Variables|Default|SetLight%20Ammo (Math|Integer|Clamp(Integer) (- (Variables|Default|GetLight%20Ammo) (Variables|Default|GetAmmoToRemove)) 0 (Variables|Default|GetMax%20Light%20Ammo))))
    (:NewEnumerator1
      (Variables|Default|SetMedium%20Ammo (Math|Integer|Clamp(Integer) (- (Variables|Default|GetMedium%20Ammo) (Variables|Default|GetAmmoToRemove)) 0 (Variables|Default|GetMax%20Medium%20Ammo))))
    (:NewEnumerator2
      (Variables|Default|SetHeavy%20Ammo (Math|Integer|Clamp(Integer) (- (Variables|Default|GetHeavy%20Ammo) (Variables|Default|GetAmmoToRemove)) 0 (Variables|Default|GetMax%20Heavy%20Ammo))))
    (:NewEnumerator3
      (Variables|Default|SetShotgun%20Ammo (Math|Integer|Clamp(Integer) (- (Variables|Default|GetShotgun%20Ammo) (Variables|Default|GetAmmoToRemove)) 0 (Variables|Default|GetMax%20Shotgun%20Ammo))))
    (:NewEnumerator4
      (Variables|Default|SetEnergy%20Ammo (Math|Integer|Clamp(Integer) (- (Variables|Default|GetEnergy%20Ammo) (Variables|Default|GetAmmoToRemove)) 0 (Variables|Default|GetMax%20Energy%20Ammo))))))

(fn GetAmmoOfType
  (params (AmmoType :type Enum_AmmoType%20Enum :default "NewEnumerator0"))
  (switch Utilities|FlowControl|Switch|SwitchonEnum_AmmoType AmmoType
    (:NewEnumerator0
      (return (!= (Variables|Default|GetLight%20Ammo) 0) (Variables|Default|GetLight%20Ammo)))
    (:NewEnumerator1
      (return (!= (Variables|Default|GetMedium%20Ammo) 0) (Variables|Default|GetMedium%20Ammo)))
    (:NewEnumerator2
      (return (!= (Variables|Default|GetHeavy%20Ammo) 0) (Variables|Default|GetHeavy%20Ammo)))
    (:NewEnumerator3
      (return (!= (Variables|Default|GetShotgun%20Ammo) 0) (Variables|Default|GetShotgun%20Ammo)))
    (:NewEnumerator4
      (return (!= (Variables|Default|GetEnergy%20Ammo) 0) (Variables|Default|GetEnergy%20Ammo)))))

(fn IsFull
  (params (AmmoType :type Enum_AmmoType%20Enum :default "NewEnumerator0"))
  (switch Utilities|FlowControl|Switch|SwitchonEnum_AmmoType AmmoType
    (:NewEnumerator0
      (return (== (Variables|Default|GetLight%20Ammo) (Variables|Default|GetMax%20Light%20Ammo))))
    (:NewEnumerator1
      (return (== (Variables|Default|GetMedium%20Ammo) (Variables|Default|GetMax%20Medium%20Ammo))))
    (:NewEnumerator2
      (return (== (Variables|Default|GetHeavy%20Ammo) (Variables|Default|GetMax%20Heavy%20Ammo))))
    (:NewEnumerator3
      (return (== (Variables|Default|GetShotgun%20Ammo) (Variables|Default|GetMax%20Shotgun%20Ammo))))
    (:NewEnumerator4
      (return (== (Variables|Default|GetEnergy%20Ammo) (Variables|Default|GetMax%20Energy%20Ammo))))))