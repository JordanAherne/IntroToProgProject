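; BP_TestOverlap is a test pickup-style trigger that destroys itself when the player character overlaps its Box, as part of opening the goal.
; After destroying itself, it checks whether any BP_TestOverlap or BP_TestInteractable actors remain in the level.
; If neither remains, it prints that the goal has opened and destroys the BP_GoalDoor it finds.
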(event OnComponentBeginOverlap(Box)
  (params (OverlappedComponent :type Primitive%20Component%20Object%20Reference) (OtherActor :type Actor%20Object%20Reference) (OtherComp :type Primitive%20Component%20Object%20Reference) (OtherBodyIndex :type Integer) (bFromSweep :type Boolean) (SweepResult :type Hit%20Result%20Structure%20%28by%20ref%29))
  (if (== OtherActor (Game|GetPlayerCharacter 0))
    (Development|PrintString "Overlapped")
    (Actor|DestroyActor)
    (bind _returnvalue (Actor|GetActorOfClass "BP_TestOverlap_C"))
    (bind _returnvalue_2 (Actor|GetActorOfClass "/Game/Production/Blueprints/BP_TestInteractable.BP_TestInteractable_C"))
    (if (not (Utilities|IsValid _returnvalue_2))
      (if (not (Utilities|IsValid _returnvalue))
        (Development|PrintString "THE GOAL HAS OPENED")
        (bind _returnvalue_3 (Actor|GetActorOfClass "/Game/Production/Blueprints/PuzzleLevelBPs/BP_GoalDoor.BP_GoalDoor_C"))
        (Actor|DestroyActor _returnvalue_3)))))

(fn ConstructionScript
  (|CallParentFunction))