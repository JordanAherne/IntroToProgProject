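; BP_Breakable is a destructible actor that takes damage, changes colour when badly hurt, and is destroyed at zero health.
; The construction script creates a dynamic material instance on the Cube mesh and applies the default colour.
; AnyDamage subtracts from clamped health, prints it for debugging, switches to the damaged colour below half health, and destroys the actor when health reaches zero.
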(event Game|Damage|EventAnyDamage
  (params (Damage :type Float%20%28single-precision%29) (DamageType :type Damage%20Type%20Object%20Reference) (InstigatedBy :type Controller%20Object%20Reference) (DamageCauser :type Actor%20Object%20Reference))
  (bind _output_get (Variables|Default|SetCurrentHealth (Math|Float|Clamp(Float) (- (Variables|Default|GetCurrentHealth) Damage) 0.0 (Variables|Default|GetMaxHealth))))
  (Development|PrintString (Utilities|String|ToString(Float) _output_get))
  (if (< (Variables|Default|GetCurrentHealth) (/ (Variables|Default|GetMaxHealth) 2.0))
    (Rendering|Material|SetVectorParameterValue (Variables|Default|GetMaterial) "DefaultColour" (Variables|Default|GetDamagedColour) :!class /Script/Engine.MaterialInstanceDynamic)
    (if (== (Variables|Default|GetCurrentHealth) 0.0)
      (Actor|DestroyActor))))

(fn ConstructionScript
  (bind _returnvalue (Rendering|Material|CreateDynamicMaterialInstance (Variables|Default|GetCube) 0 0 "None" :!class /Script/Engine.PrimitiveComponent))
  (bind _output_get (Variables|Default|SetMaterial _returnvalue))
  (Rendering|Material|SetVectorParameterValue _output_get "DefaultColour" (Variables|Default|GetDefaultColour) :!class /Script/Engine.MaterialInstanceDynamic))