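; BP_TelePad is a teleport pad that sends the first-person shooter character to a linked DestinationPad after a countdown.
; Beginning overlap shows a WBP_TeleportCountdown widget and starts a timer using its Countdown value.
; When the timer fires, the character moves to the destination's SpawnPoint with zeroed rotation and the Teleported dispatcher is called.
; Any actor ending overlap cancels the timer and removes the widget, without a character check.
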(event Custom|Teleport
  (Transformation|Teleport (stale Collision|EventActorBeginOverlap OtherActor) (Transformation|GetWorldLocation (Variables|/Game/Production/Blueprints/LevelComponents/BP_DestinationPad.BP_DestinationPad_C|GetSpawnPoint (Variables|Default|GetDestinationPad))) "0, 0, 0")
  (Default|CallTeleported))

(event Collision|EventActorEndOverlap
  (params (OtherActor :type Actor%20Object%20Reference))
  (Utilities|Time|ClearandInvalidateTimerbyHandle (stale Collision|EventActorBeginOverlap _returnvalue_2))
  (Widget|RemovefromParent (Variables|Default|GetTimerPrompt)))

(event Collision|EventActorBeginOverlap
  (params (OtherActor :type Actor%20Object%20Reference))
  (Utilities|Casting|CastToBP_FirstPersonShooterCharacter OtherActor)
  (bind _returnvalue (UserInterface|CreateWidget "/Game/Production/Blueprints/WBP/WBP_TeleportCountdown.WBP_TeleportCountdown_C"))
  (bind _output_get (Variables|Default|SetTimerPrompt _returnvalue))
  (UserInterface|Viewport|AddtoViewport _output_get 0)
  (bind _returnvalue_2 (Utilities|Time|SetTimerbyEvent (delegate Custom|Teleport) (Variables|/Game/Production/Blueprints/WBP/WBP_TeleportCountdown.WBP_TeleportCountdown_C|GetCountdown (Variables|Default|GetTimerPrompt)))))

(fn ConstructionScript)