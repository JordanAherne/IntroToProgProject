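; BP_LockedDoor is a locked door that a key card reader opens and closes.
; On BeginPlay it finds a single BP_KeyCardReader by class and binds its Toggle event to that reader's door-toggle dispatcher.
; Toggle flips the Cube's visibility and switches its collision between QueryAndPhysics and NoCollision.
; Interacting with the door directly only prints a locked message and returns true.
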(event Custom|Toggle
  (bind _cube (Variables|Default|GetCube))
  (bind _cube_2 (Variables|Default|GetCube))
  (Rendering|ToggleVisibility _cube false)
  (if (Utilities|Enum|Equal(Enum) (Collision|GetCollisionEnabled _cube) "QueryAndPhysics")
    (Collision|SetCollisionEnabled _cube_2 "NoCollision")
    (else
      (Collision|SetCollisionEnabled _cube_2 "QueryAndPhysics"))))

(event EventBeginPlay
  (bind _returnvalue (Actor|GetActorOfClass "/Game/Production/Blueprints/LevelComponents/BP_KeyCardReader.BP_KeyCardReader_C"))
  (bind _output_get (Variables|Default|SetCardReader _returnvalue))
  (EventDispatchers|BindEventtoToggleDoor _output_get (delegate Custom|Toggle)))

(event Collision|EventActorBeginOverlap
  (params (OtherActor :type Actor%20Object%20Reference)))

(fn ConstructionScript)

(fn Interact
  (params (Interractor :type Character%20Object%20Reference))
  (Development|PrintString "LOCKED")
  (return true))