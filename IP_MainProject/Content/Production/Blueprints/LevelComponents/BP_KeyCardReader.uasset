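; BP_KeyCardReader is an interactable card reader that unlocks linked doors once a key card has been collected.
; The CardCollected event sets a HasKeyCard flag on the reader itself.
; Interact checks that flag, then either swaps the Cube1 material to the open look and calls Unlock on every Door entry, or prints a need-key message.
; Interact returns true in both cases.
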(event Custom|CardCollected
  (Variables|Default|SethasKeyCard true))

(event EventBeginPlay)

(event Collision|EventActorBeginOverlap
  (params (OtherActor :type Actor%20Object%20Reference)))

(event EventTick
  (params (DeltaSeconds :type Float%20%28single-precision%29)))

(fn ConstructionScript)

(fn Interact
  (params (Interractor :type Character%20Object%20Reference))
  (if (Variables|Default|GethasKeyCard)
    (Rendering|Material|SetMaterial (Variables|Default|GetCube1) 0 "/Game/Production/Materials/M_CardReaderOpen.M_CardReaderOpen")
    (for _array_element (Variables|Default|GetDoor)
      (Default|Unlock _array_element))
    (else
      (Development|PrintString "Need Key")))
  (return true))