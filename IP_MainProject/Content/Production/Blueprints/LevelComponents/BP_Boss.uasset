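; BP_Boss is a turret boss that tracks and shoots the first-person player when its pawn sensing spots them.
; It interpolates its aim toward the player and fires a child-actor gun from the right shoot point, shortening fire delay per call.
; After 100 calls it sets a cooldown, never cleared here.
; On death it tilts its body and exposes its heart, then retracts the heart and clears the dead flag after timed delays.
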(event OnSeePawn(PawnSensing)
  (params (Pawn :type Pawn%20Object%20Reference))
  (if (not (Variables|/Game/Production/Blueprints/Components/BPC_Health.BPC_Health_C|GetDead (Variables|Default|GetBPC_Health)))
    (bind _asbp_first_person_shooter_character (Utilities|Casting|CastToBP_FirstPersonShooterCharacter Pawn))
    (bind _output_get (Variables|Default|SetPlayer _asbp_first_person_shooter_character))
    (CallFunction|TargetPlayer _output_get)
    (CallFunction|ShootTurrent (Variables|Default|GetRTurret) (Variables|Default|GetRShootPoint))))

(event OnDeath(BPC_Health)
  (CallFunction|Offline)
  (Utilities|FlowControl|Delay 5.0)
  (CallFunction|Online)
  (Utilities|FlowControl|Delay 5.0)
  (Variables|/Game/Production/Blueprints/Components/BPC_Health.BPC_Health_C|SetDead (Variables|Default|GetBPC_Health) false))

(event Custom|Offline
  (bind _heart (Variables|Default|GetHeart))
  (bind _bodypivot (Variables|Default|GetBodyPivot))
  (bind _relativelocation (Variables|/Script/Engine.SceneComponent|GetRelativeLocation _heart))
  (Components|MoveComponentTo _bodypivot (Variables|/Script/Engine.SceneComponent|GetRelativeLocation _bodypivot) (Variables|Default|GetOfflineRotation) false false 2.0 false)
  (Components|MoveComponentTo _heart (Math|Vector|MakeVector (Variables|Default|GetExposedHeartPosition) (.y _relativelocation) (.z _relativelocation)) (Variables|/Script/Engine.SceneComponent|GetRelativeRotation _heart) false false 2.0 false))

(event Custom|Online
  (bind _heart (Variables|Default|GetHeart))
  (bind _bodypivot (Variables|Default|GetBodyPivot))
  (Components|MoveComponentTo _heart (Variables|Default|GetDefaultHeartPosition) (Variables|/Script/Engine.SceneComponent|GetRelativeRotation _heart) false false 2.0 false)
  (Components|MoveComponentTo _bodypivot (Variables|/Script/Engine.SceneComponent|GetRelativeLocation _bodypivot) "0, 0, 0" false false 2.0 false))

(event EventBeginPlay
  (Variables|Default|SetDefaultHeartPosition (Variables|/Script/Engine.SceneComponent|GetRelativeLocation (Variables|Default|GetHeart)))
  (bind _asbp_boss_turret_gun (Utilities|Casting|CastToBP_BossTurretGun (Variables|/Script/Engine.ChildActorComponent|GetChildActor (Variables|Default|GetGun))))
  (Variables|Default|SetAs%20BP%20Boss%20Turret%20Gun _asbp_boss_turret_gun))

(event Game|Damage|EventAnyDamage
  (params (Damage :type Float%20%28single-precision%29) (DamageType :type Damage%20Type%20Object%20Reference) (InstigatedBy :type Controller%20Object%20Reference) (DamageCauser :type Actor%20Object%20Reference))
  (Default|HealthUpdate (Variables|Default|GetBPC_Health) Damage))

(fn ConstructionScript)

(fn TargetPlayer
  (params (Player :type Actor%20Object%20Reference))
  (bind _returnvalue (Utilities|Time|GetWorldDeltaSeconds))
  (bind _returnvalue_2 (Transformation|GetActorLocation Player))
  (bind _rotationspeed (Variables|Default|GetRotationSpeed))
  (bind _cylinder (Variables|Default|GetCylinder))
  (bind _returnvalue_3 (Transformation|GetWorldRotation _cylinder))
  (bind _returnvalue_4 (Transformation|GetWorldLocation _cylinder))
  (bind _returnvalue_5 (Math|Rotator|FindLookatRotation _returnvalue_4 _returnvalue_2))
  (bind _returnvalue_6 (Math|Interpolation|RInterpTo _returnvalue_3 _returnvalue_5 _returnvalue _rotationspeed))
  (Transformation|SetRelativeRotation (Variables|Default|GetBodyPivot) (Math|Rotator|MakeRotator 0.0 (.pitch _returnvalue_6) 0.0) false false)
  (Transformation|SetActorRotation (Math|Rotator|MakeRotator 0.0 (.pitch _returnvalue_6) (.yaw _returnvalue_6))))

(fn ShootTurrent
  (params (Turret :type Scene%20Component%20Object%20Reference) (ShootPoint :type Scene%20Component%20Object%20Reference))
  (bind _as_bp_boss_turret_gun (Variables|Default|GetAs%20BP%20Boss%20Turret%20Gun))
  (LocalVariables|SetLocalTurret Turret)
  (if (not (Variables|Default|GetCooldown))
    (Default|Shoot (Variables|Default|GetAs%20BP%20Boss%20Turret%20Gun) (Transformation|GetWorldLocation ShootPoint) (Math|Vector|GetForwardVector ShootPoint))
    (Variables|/Game/Production/Blueprints/Weapons/BP_WeaponBase.BP_WeaponBase_C|SetFireDelay _as_bp_boss_turret_gun (* (Variables|/Game/Production/Blueprints/Weapons/BP_WeaponBase.BP_WeaponBase_C|GetFireDelay _as_bp_boss_turret_gun) 0.9))
    (bind _result (Math|Integer|IncrementInt (Variables|Default|GetCounter))
      (:%20%20
        (Development|PrintString (Utilities|String|ToString(Integer) _result))
        (if (>= _result 100)
          (Variables|Default|SetCooldown true)
          (Variables|Default|SetCounter 0)
          (Variables|/Game/Production/Blueprints/Weapons/BP_WeaponBase.BP_WeaponBase_C|SetFireDelay (Variables|Default|GetAs%20BP%20Boss%20Turret%20Gun) (Variables|Default|GetOriginalFireDelay)))))))