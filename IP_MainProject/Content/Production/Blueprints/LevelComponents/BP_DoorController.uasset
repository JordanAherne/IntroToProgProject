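; BP_DoorController is an interactable level component that toggles a linked Door and Payload.
; Interact fires the Opeened dispatcher on every use, then opens or closes the Door based on its IsOpen state.
; It then independently flips the Payload between active and inactive based on IsActive, and always returns false.
; The event graph and construction script are empty, so all logic lives in Interact.
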(event EventBeginPlay)

(event Collision|EventActorBeginOverlap
  (params (OtherActor :type Actor%20Object%20Reference)))

(event EventTick
  (params (DeltaSeconds :type Float%20%28single-precision%29)))

(fn ConstructionScript)

(fn Interact
  (params (Interractor :type Character%20Object%20Reference))
  (bind _door (Variables|Default|GetDoor))
  (bind _payload (Variables|Default|GetPayload))
  (Default|CallOpeened)
  (if (Variables|/Game/Production/Blueprints/LevelComponents/BP_RisingDoor.BP_RisingDoor_C|GetisOpen (Variables|Default|GetDoor))
    (Default|Close _door)
    (else
      (Default|Open _door)))
  (if (Variables|/Game/Production/Blueprints/LevelComponents/BP_Payload.BP_Payload_C|GetisActive (Variables|Default|GetPayload))
    (Default|Inactive _payload)
    (else
      (Default|Active _payload)))
  (return false))