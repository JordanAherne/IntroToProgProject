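; A lockable door Blueprint that players open and close by interacting with it.
; A timeline lerps the mesh's yaw from zero to a configurable open angle, playing forward to open and in reverse to close.
; Interact toggles the door only when it is unlocked, while Unlock clears the lock, opens the door and fires an Unlocked call.
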(event Custom|Open
  (Variables|Default|SetdoorOpen true)
  (bind _doorrotation (Timeline|Timeline Play)
    (:Update
      (Transformation|SetRelativeRotation (Variables|Default|GetMesh) (Math|Rotator|MakeRotator 0.0 0.0 (Math|Float|Lerp 0.0 (Variables|Default|GetDoorOpenAngle) _doorrotation)) false false))))

(event Custom|Close
  (Variables|Default|SetdoorOpen false)
  (bind _doorrotation (Timeline|Timeline Reverse)
    (:Update
      (Transformation|SetRelativeRotation (Variables|Default|GetMesh) (Math|Rotator|MakeRotator 0.0 0.0 (Math|Float|Lerp 0.0 (Variables|Default|GetDoorOpenAngle) _doorrotation)) false false))))

(event Custom|Unlock
  (if (Variables|Default|Getlocked)
    (Variables|Default|Setlocked false)
    (CallFunction|Open)
    (Default|CallUnlocked)))

(fn ConstructionScript)

(fn Interact
  (params (Interractor :type Character%20Object%20Reference))
  (if (not (Variables|Default|Getlocked))
    (if (Variables|Default|GetdoorOpen)
      (CallFunction|Close)
      (else
        (CallFunction|Open)))
    (return false)))