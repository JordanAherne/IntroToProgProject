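; Level actor that recharges grenade launcher ammo while the first-person character stands inside its cylinder.
; Activate and Deactivate toggle the cylinder's visibility and sphere's material, and charging only begins while active.
; Entering with a grenade launcher starts a timer based on its reload time and shows a progress widget.
; Each completion adds one round and restarts until full; leaving clears the timer and widget unless Hidden is set.
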(event OnComponentBeginOverlap(Cylinder)
  (params (OverlappedComponent :type Primitive%20Component%20Object%20Reference) (OtherActor :type Actor%20Object%20Reference) (OtherComp :type Primitive%20Component%20Object%20Reference) (OtherBodyIndex :type Integer) (bFromSweep :type Boolean) (SweepResult :type Hit%20Result%20Structure%20%28by%20ref%29))
  (if (Variables|Default|GetisActive)
    (bind _asbp_first_person_shooter_character (Utilities|Casting|CastToBP_FirstPersonShooterCharacter OtherActor))
    (bind _output_get (Variables|Default|SetPlayer _asbp_first_person_shooter_character))
    (bind _asbp_grenade_launcher (Utilities|Casting|CastToBP_GrenadeLauncher (Variables|/Game/Production/Blueprints/BP_FirstPersonShooterCharacter.BP_FirstPersonShooterCharacter_C|GetCurrentWeapon _output_get)))
    (Variables|Default|SetGrenadeLauncher _asbp_grenade_launcher)
    (CallFunction|ChargeWeapon)))

(event OnComponentEndOverlap(Cylinder)
  (params (OverlappedComponent :type Primitive%20Component%20Object%20Reference) (OtherActor :type Actor%20Object%20Reference) (OtherComp :type Primitive%20Component%20Object%20Reference) (OtherBodyIndex :type Integer))
  (Utilities|Casting|CastToBP_FirstPersonShooterCharacter OtherActor)
  (if (not (Variables|Rendering|GetbHidden))
    (Utilities|Time|ClearandInvalidateTimerbyHandle (Variables|Default|GetTimer))
    (Widget|RemovefromParent (Variables|Default|GetProgressBar))))

(event Custom|Deactivate
  (bind _output_get (Variables|Default|SetisActive false))
  (Rendering|SetVisibility (Variables|Default|GetCylinder) _output_get false)
  (Rendering|Material|SetMaterial (Variables|Default|GetSphere) 0 "/Game/Production/Blueprints/PuzzleLevelBPs/NewMaterial.NewMaterial"))

(event Custom|Activate
  (bind _output_get (Variables|Default|SetisActive true))
  (Rendering|SetVisibility (Variables|Default|GetCylinder) _output_get false)
  (Rendering|Material|SetMaterial (Variables|Default|GetSphere) 0 "/Game/Production/Materials/M_BlueEmissive.M_BlueEmissive"))

(event Custom|AddAmmo
  (Utilities|Time|ClearandInvalidateTimerbyHandle (Variables|Default|GetTimer))
  (Widget|RemovefromParent (Variables|Default|GetProgressBar))
  (Default|AddAmmo (Variables|/Game/Production/Blueprints/BP_FirstPersonShooterCharacter.BP_FirstPersonShooterCharacter_C|GetBPC_AmmoInventory (Variables|Default|GetPlayer)) 1 "NewEnumerator4")
  (CallFunction|ChargeWeapon))

(event Custom|ChargeWeapon
  (bind _isfull (Default|IsFull (Variables|/Game/Production/Blueprints/BP_FirstPersonShooterCharacter.BP_FirstPersonShooterCharacter_C|GetBPC_AmmoInventory (Variables|Default|GetPlayer)) "NewEnumerator4"))
  (if (not _isfull)
    (if (Utilities|Time|IsValidTimerHandle (Variables|Default|GetTimer))
      ;[0.15 0.15 0.15 0.5] If there is already a Timer, unpause it and add ProgressBar to Viewport
      (Utilities|Time|UnpauseTimerbyHandle (Variables|Default|GetTimer))
      (UserInterface|Viewport|AddtoViewport (Variables|Default|GetProgressBar) 0)
      (else
        ;[0.15 0.15 0.15 0.5] Create and add Progress bar to Viewport
        (bind _returnvalue (UserInterface|CreateWidget "/Game/Production/Blueprints/Objectives/UI/WBP_CaptureProgress.WBP_CaptureProgress_C"))
        (bind _output_get (Variables|Default|SetProgressBar _returnvalue))
        (UserInterface|Viewport|AddtoViewport _output_get 0)
        (bind _output_get_2 (Variables|/Game/Production/Blueprints/Objectives/UI/WBP_CaptureProgress.WBP_CaptureProgress_C|SetMaxProgress (Variables|Default|GetProgressBar) (Variables|/Game/Production/Blueprints/Weapons/BP_WeaponBase.BP_WeaponBase_C|GetReloadTime (Variables|Default|GetGrenadeLauncher))))
        (bind _returnvalue_2 (Utilities|Time|SetTimerbyEvent (delegate Custom|AddAmmo) _output_get_2))
        (Variables|Default|SetTimer _returnvalue_2)))))

(event EventBeginPlay
  (bind _sphere (Variables|Default|GetSphere))
  (bind _cylinder (Variables|Default|GetCylinder))
  (if (Variables|Default|GetisActive)
    (Rendering|SetVisibility _cylinder true false)
    (Rendering|Material|SetMaterial _sphere 0 "/Game/Production/Materials/M_BlueEmissive.M_BlueEmissive")
    (else
      (Rendering|SetVisibility _cylinder false false)
      (Rendering|Material|SetMaterial _sphere 0 "/Game/Production/Blueprints/PuzzleLevelBPs/NewMaterial.NewMaterial"))))

(event Collision|EventActorBeginOverlap
  (params (OtherActor :type Actor%20Object%20Reference)))

(event EventTick
  (params (DeltaSeconds :type Float%20%28single-precision%29)))

(fn ConstructionScript)