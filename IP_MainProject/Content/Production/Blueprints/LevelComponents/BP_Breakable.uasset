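; BP_Breakable is a damageable crate that swaps to a damaged material at half health and drops a pickup when destroyed.
; BPCHealth tracks damage, and its OnDeath spawns loot at the cube before destroying the actor.
; Flags select random loot, health, ammo (optionally randomly typed) or the first Loot entry.
; Random loot rolls one past the array length, allowing no drop, and re-rolls at each check.
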(event OnDeath(BPC_Health)
  (bind _loot (Variables|Default|GetLoot))
  (bind _loot_2 (Variables|Default|GetLoot))
  (bind _returnvalue (Utilities|Array|Length _loot))
  (bind _returnvalue_2 (+ _returnvalue 1))
  (bind _returnvalue_3 (Math|Random|RandomInteger _returnvalue_2))
  (bind _output (Utilities|Array|Get(acopy) _loot_2 _returnvalue_3))
  (if (Variables|Default|GetRandomLoot?)
    (if (Utilities|IsValidClass _output)
      (if (Utilities|ClassIsChildOf _output "/Game/Production/Blueprints/LevelComponents/Pickups/BP_AmmoPickup.BP_AmmoPickup_C")
        (Game|SpawnActorfromClass "/Game/Production/Blueprints/LevelComponents/Pickups/BP_AmmoPickup.BP_AmmoPickup_C" (Math|Transform|MakeTransform (Transformation|GetWorldLocation (Variables|Default|GetCube)) "0, 0, 0" "1.000000,1.000000,1.000000") "Undefined" "MultiplyWithRoot" 0 (Variables|Default|GetAmmoType) 20 0)
        (else
          (Game|SpawnActorfromClass _output (Math|Transform|MakeTransform (Transformation|GetWorldLocation (Variables|Default|GetCube)) "0, 0, 0" "1.000000,1.000000,1.000000") "Undefined" "MultiplyWithRoot" 0 0)))
      (Actor|DestroyActor)
      (else
        (Actor|DestroyActor)))
    (elif (Variables|Default|GetHealthOnly?)
      (Game|SpawnActorfromClass "/Game/Production/Blueprints/LevelComponents/Pickups/BP_HealthPickup.BP_HealthPickup_C" (Math|Transform|MakeTransform (Transformation|GetWorldLocation (Variables|Default|GetCube)) "0, 0, 0" "1.000000,1.000000,1.000000") "Undefined" "MultiplyWithRoot" 0 0)
      (Actor|DestroyActor)
      (elif (Variables|Default|GetAmmoOnly?)
        (if (Variables|Default|GetRandomAmmoType?)
          (bind _enumvalue (|ForEachEnum_AmmoType)
            (:LoopBody
              (if (== (Math|Random|RandomInteger 4) (Variables|Default|GetCounter))
                (Variables|Default|SetAmmoType _enumvalue)
                (else
                  (Math|Integer|IncrementInt (Variables|Default|GetCounter)))))
            (:then
              (Game|SpawnActorfromClass "/Game/Production/Blueprints/LevelComponents/Pickups/BP_AmmoPickup.BP_AmmoPickup_C" (Math|Transform|MakeTransform (Transformation|GetWorldLocation (Variables|Default|GetCube)) "0, 0, 0" "1.000000,1.000000,1.000000") "Undefined" "MultiplyWithRoot" 0 (Variables|Default|GetAmmoType) 20 0)
              (Actor|DestroyActor)))
          (else
            (Game|SpawnActorfromClass "/Game/Production/Blueprints/LevelComponents/Pickups/BP_AmmoPickup.BP_AmmoPickup_C" (Math|Transform|MakeTransform (Transformation|GetWorldLocation (Variables|Default|GetCube)) "0, 0, 0" "1.000000,1.000000,1.000000") "Undefined" "MultiplyWithRoot" 0 (Variables|Default|GetAmmoType) 20 0)
            (Actor|DestroyActor)))
        (else
          (Game|SpawnActorfromClass (Utilities|Array|Get(acopy) (Variables|Default|GetLoot)) (Math|Transform|MakeTransform (Transformation|GetWorldLocation (Variables|Default|GetCube)) "0, 0, 0" "1.000000,1.000000,1.000000") "Undefined" "MultiplyWithRoot" 0 0)
          (Actor|DestroyActor))))))

(event Game|Damage|EventAnyDamage
  (params (Damage :type Float%20%28single-precision%29) (DamageType :type Damage%20Type%20Object%20Reference) (InstigatedBy :type Controller%20Object%20Reference) (DamageCauser :type Actor%20Object%20Reference))
  (bind _bpc_health (Variables|Default|GetBPC_Health))
  (bind _currenthealth (Default|TakeHealth _bpc_health Damage))
  (Utilities|IsValid (Variables|Default|GetBPC_Health)
    (:Is%20Valid
      (if (<= _currenthealth (/ (Variables|/Game/Production/Blueprints/Components/BPC_Health.BPC_Health_C|GetMaxHealth _bpc_health) 2.0))
        (Rendering|Material|SetMaterial (Variables|Default|GetCube) 0 "/Game/Production/Materials/M_DamagedCrate.M_DamagedCrate")))))

(fn ConstructionScript)