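; BP_Payload is an escort-style payload that travels through checkpoints while active, moving when the player enters its sphere and stopping when they leave.
; Each leg's duration comes from 2D distance over Speed, and completed legs turn the base toward the next checkpoint.
; The final checkpoint fires DestinationReached, hides the beams, lowers the base and clears immunity.
; Unless immune, it passes damage to a health component, whose death event spawns a large explosion, calls Exploded and destroys it.
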(event OnDeath(BPC_Health)
  (Game|SpawnActorfromClass "/Game/Production/Blueprints/LevelComponents/BP_Explosion.BP_Explosion_C" (Transformation|GetActorTransform self) "Undefined" "MultiplyWithRoot" 0 2e+01 0)
  (Default|CallExploded)
  (Actor|DestroyActor))

(event OnComponentBeginOverlap(Sphere)
  (params (OverlappedComponent :type Primitive%20Component%20Object%20Reference) (OtherActor :type Actor%20Object%20Reference) (OtherComp :type Primitive%20Component%20Object%20Reference) (OtherBodyIndex :type Integer) (bFromSweep :type Boolean) (SweepResult :type Hit%20Result%20Structure%20%28by%20ref%29))
  (bind _asbp_first_person_shooter_character (Utilities|Casting|CastToBP_FirstPersonShooterCharacter OtherActor))
  (Variables|Default|SetPlayer _asbp_first_person_shooter_character)
  (if (Variables|Default|GetisActive)
    (CallFunction|Move)))

(event OnComponentEndOverlap(Sphere)
  (params (OverlappedComponent :type Primitive%20Component%20Object%20Reference) (OtherActor :type Actor%20Object%20Reference) (OtherComp :type Primitive%20Component%20Object%20Reference) (OtherBodyIndex :type Integer))
  (bind _asbp_first_person_shooter_character (Utilities|Casting|CastToBP_FirstPersonShooterCharacter OtherActor))
  (Variables|Default|SetPlayer _asbp_first_person_shooter_character)
  (if (Variables|Default|GetisActive)
    (CallFunction|Stop)))

(event Custom|Active
  (Rendering|SetVisibility (Variables|Default|GetBeam1) true false)
  (Components|MoveComponentTo (Variables|Default|GetBase) "0, 0, 0" "0, 0, 0" false true 2.0 false)
  (Variables|Default|SetisActive true))

(event Custom|Inactive
  (bind _base (Variables|Default|GetBase))
  (bind _relativelocation (Variables|/Script/Engine.SceneComponent|GetRelativeLocation _base))
  (Variables|Default|SetisActive false)
  (Rendering|SetVisibility (Variables|Default|GetBeam2) false false)
  (Components|MoveComponentTo _base (Math|Vector|MakeVector (.x _relativelocation) (.y _relativelocation) (- (.z _relativelocation) 1e+02)) (Variables|/Script/Engine.SceneComponent|GetRelativeRotation _base) false false 2.0 false))

(event Custom|Move
  (bind _base (Variables|Default|GetBase))
  (bind _base_2 (Variables|Default|GetBase))
  (bind _relativelocation (Variables|/Script/Engine.SceneComponent|GetRelativeLocation _base))
  (Components|MoveComponentTo _base_2 (Utilities|Array|Get(acopy) (Variables|Default|GetCheckpoints) (Variables|Default|GetCheckpoint)) (Variables|/Script/Engine.SceneComponent|GetRelativeRotation _base_2) false false (Variables|Default|GetOver%20Time) false)
  (CallFunction|CalcOverTime)
  (if (Utilities|AtCheckpoint?)
    (bind _result (Math|Integer|IncrementInt (Variables|Default|GetCheckpoint))
      (:%20%20
        (if (not (>= _result (Utilities|Array|Length (Variables|Default|GetCheckpoints))))
          (Components|MoveComponentTo _base _relativelocation (Math|Rotator|FindLookatRotation _relativelocation (Utilities|Array|Get(acopy) (Variables|Default|GetCheckpoints) (Variables|Default|GetCheckpoint))) false false (Variables|Default|GetRotationDuration) false)
          (CallFunction|CalcOverTime)
          (CallFunction|Move)
          (else
            (Default|CallDestinationReached)
            (CallFunction|Inactive)
            (Variables|Default|Setimune false)))))))

(event Custom|Stop
  (bind _base (Variables|Default|GetBase))
  (bind _base_2 (Variables|Default|GetBase))
  (bind _relativelocation (Variables|/Script/Engine.SceneComponent|GetRelativeLocation _base))
  (Components|MoveComponentTo _base_2 (Utilities|Array|Get(acopy) (Variables|Default|GetCheckpoints) (Variables|Default|GetCheckpoint)) (Variables|/Script/Engine.SceneComponent|GetRelativeRotation _base_2) false false (Variables|Default|GetOver%20Time) false) ; enters at Stop
)

(event EventBeginPlay
  (CallFunction|CalcOverTime)
  (if (Variables|Default|GetisActive)
    (CallFunction|Active)
    (else
      (CallFunction|Inactive))))

(event Collision|EventActorBeginOverlap
  (params (OtherActor :type Actor%20Object%20Reference)))

(event EventTick
  (params (DeltaSeconds :type Float%20%28single-precision%29)))

(event Game|Damage|EventAnyDamage
  (params (Damage :type Float%20%28single-precision%29) (DamageType :type Damage%20Type%20Object%20Reference) (InstigatedBy :type Controller%20Object%20Reference) (DamageCauser :type Actor%20Object%20Reference))
  (if (not (Variables|Default|Getimune))
    (Default|HealthUpdate (Variables|Default|GetBPC_Health) Damage)))

(fn ConstructionScript)

(fn CalcOverTime
  (bind _base (Variables|Default|GetBase))
  (bind _checkpoints (Variables|Default|GetCheckpoints))
  (bind _checkpoint (Variables|Default|GetCheckpoint))
  (bind _output (Utilities|Array|Get(acopy) _checkpoints _checkpoint))
  (bind _relativelocation (Variables|/Script/Engine.SceneComponent|GetRelativeLocation _base))
  (Variables|Default|SetOver%20Time (/ (Math|Vector|Distance2D(Vector) (Math|Vector2D|MakeVector2D (.x _output) (.y _output)) (Math|Vector2D|MakeVector2D (.x _relativelocation) (.y _relativelocation))) (Variables|Default|GetSpeed))))