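; Health pickup that floats in the level and heals the first-person shooter character on overlap.
; A timeline started at BeginPlay lerps the cube's relative Z between minimum and maximum float heights.
; On box overlap, if current health differs from max, it passes HealValue through ApplyDamage rather than a dedicated heal function.
; It then calls HealthPickup and destroys itself.
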(event OnComponentBeginOverlap(Box)
  (params (OverlappedComponent :type Primitive%20Component%20Object%20Reference) (OtherActor :type Actor%20Object%20Reference) (OtherComp :type Primitive%20Component%20Object%20Reference) (OtherBodyIndex :type Integer) (bFromSweep :type Boolean) (SweepResult :type Hit%20Result%20Structure%20%28by%20ref%29))
  (bind _asbp_first_person_shooter_character (Utilities|Casting|CastToBP_FirstPersonShooterCharacter OtherActor))
  (if (!= (Variables|/Game/Production/Blueprints/Components/BPC_Health.BPC_Health_C|GetCurrentHealth (Variables|/Game/Production/Blueprints/BP_FirstPersonShooterCharacter.BP_FirstPersonShooterCharacter_C|GetBPC_Health _asbp_first_person_shooter_character)) (Variables|/Game/Production/Blueprints/Components/BPC_Health.BPC_Health_C|GetMaxHealth (Variables|/Game/Production/Blueprints/BP_FirstPersonShooterCharacter.BP_FirstPersonShooterCharacter_C|GetBPC_Health _asbp_first_person_shooter_character)))
    (Game|Damage|ApplyDamage _asbp_first_person_shooter_character (Variables|Default|GetHealValue) 0 0)
    (Default|CallHealthPickup)
    (Actor|DestroyActor)))

(event EventBeginPlay
  (bind _float (Timeline|Floating%20Object Play)
    (:Update
      (Transformation|SetRelativeLocation (Variables|Default|GetCube) (Math|Vector|MakeVector 0.0 0.0 (Math|Float|Lerp (Variables|Default|GetFloatHeightMin) (Variables|Default|GetFloatHeightMax) _float)) false false))))

(fn ConstructionScript)