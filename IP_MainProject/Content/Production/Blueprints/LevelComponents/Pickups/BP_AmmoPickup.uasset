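; BP_AmmoPickup is a floating ammo pickup that refills the player's ammo inventory for its ammo type.
; On BeginPlay a timeline moves the cube between two heights and the cube's material is set by ammo type.
; On box overlap with the first-person shooter character, it adds ammo if that type isn't full, calls PickedUp and destroys itself.
; The construction script creates a green-tinted dynamic material, which the type-specific material replaces at runtime.
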(event OnComponentBeginOverlap(Box)
  (params (OverlappedComponent :type Primitive%20Component%20Object%20Reference) (OtherActor :type Actor%20Object%20Reference) (OtherComp :type Primitive%20Component%20Object%20Reference) (OtherBodyIndex :type Integer) (bFromSweep :type Boolean) (SweepResult :type Hit%20Result%20Structure%20%28by%20ref%29))
  (bind _asbp_first_person_shooter_character (Utilities|Casting|CastToBP_FirstPersonShooterCharacter OtherActor))
  ;[0.15 0.15 0.15 0.5] Only pick up if ammo is not full
  (bind _isfull (Default|IsFull (Variables|/Game/Production/Blueprints/BP_FirstPersonShooterCharacter.BP_FirstPersonShooterCharacter_C|GetBPC_AmmoInventory _asbp_first_person_shooter_character) (Variables|Default|GetAmmoType)))
  (if (not _isfull)
    (Default|AddAmmo (Variables|/Game/Production/Blueprints/BP_FirstPersonShooterCharacter.BP_FirstPersonShooterCharacter_C|GetBPC_AmmoInventory _asbp_first_person_shooter_character) (Variables|Default|GetAmmoValue) (Variables|Default|GetAmmoType))
    (Default|CallPickedUp)
    (Actor|DestroyActor)))

(event EventBeginPlay
  (Utilities|FlowControl|Sequence
    (:then_0
      (bind _float (Timeline|Timeline Play)
        (:Update
          (Transformation|SetRelativeLocation (Variables|Default|GetCube) (Math|Vector|MakeVector 0.0 0.0 (Math|Float|Lerp (Variables|Default|GetFloatHeightMin) (Variables|Default|GetFloatHeightMax) _float)) false false))))
    (:then_1
      (switch Utilities|FlowControl|Switch|SwitchonEnum_AmmoType (Variables|Default|GetAmmoType)
        (:NewEnumerator0
          (Rendering|Material|SetMaterial (Variables|Default|GetCube) 0 (Variables|Default|GetLightAmmoM)))
        (:NewEnumerator1
          (Rendering|Material|SetMaterial (Variables|Default|GetCube) 0 (Variables|Default|GetMedAmmoM)))
        (:NewEnumerator2
          (Rendering|Material|SetMaterial (Variables|Default|GetCube) 0 (Variables|Default|GetHeavyAmmoM)))
        (:NewEnumerator3
          (Rendering|Material|SetMaterial (Variables|Default|GetCube) 0 (Variables|Default|GetShotgunAmmoM)))))))

(event Collision|EventActorBeginOverlap
  (params (OtherActor :type Actor%20Object%20Reference)))

(event EventTick
  (params (DeltaSeconds :type Float%20%28single-precision%29)))

(fn ConstructionScript
  (bind _returnvalue (Rendering|Material|CreateDynamicMaterialInstance (Variables|Default|GetCube) 0 0 "None" :!class /Script/Engine.PrimitiveComponent))
  (bind _output_get (Variables|Default|SetMaterial _returnvalue))
  (Rendering|Material|SetVectorParameterValue _output_get "DefaultColour" "(R=0.000000,G=0.265625,B=0.000000,A=1.000000)" :!class /Script/Engine.MaterialInstanceDynamic))