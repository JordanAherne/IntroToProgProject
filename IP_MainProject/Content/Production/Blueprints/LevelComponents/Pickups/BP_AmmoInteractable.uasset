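; Ammo pickup that gives the first-person shooter character ammo of a set type and amount on interaction.
; Interact adds the ammo to the character's ammo inventory only if that type is not full, then calls PickedUp and destroys itself.
; The construction script creates a green-tinted dynamic material on the cube, which BeginPlay replaces with a material matching the ammo type.
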(event EventBeginPlay
  (switch Utilities|FlowControl|Switch|SwitchonEnum_AmmoType (Variables|Default|GetAmmoType)
    (:NewEnumerator0
      (Rendering|Material|SetMaterial (Variables|Default|GetCube) 0 (Variables|Default|GetLightAmmoM)))
    (:NewEnumerator1
      (Rendering|Material|SetMaterial (Variables|Default|GetCube) 0 (Variables|Default|GetMedAmmoM)))
    (:NewEnumerator2
      (Rendering|Material|SetMaterial (Variables|Default|GetCube) 0 (Variables|Default|GetHeavyAmmoM)))
    (:NewEnumerator3
      (Rendering|Material|SetMaterial (Variables|Default|GetCube) 0 (Variables|Default|GetShotgunAmmoM)))))

(event Collision|EventActorBeginOverlap
  (params (OtherActor :type Actor%20Object%20Reference)))

(event EventTick
  (params (DeltaSeconds :type Float%20%28single-precision%29)))

(fn ConstructionScript
  (bind _returnvalue (Rendering|Material|CreateDynamicMaterialInstance (Variables|Default|GetCube) 0 0 "None" :!class /Script/Engine.PrimitiveComponent))
  (bind _output_get (Variables|Default|SetMaterial _returnvalue))
  (Rendering|Material|SetVectorParameterValue _output_get "DefaultColour" "(R=0.000000,G=0.265625,B=0.000000,A=1.000000)" :!class /Script/Engine.MaterialInstanceDynamic))

(fn Interact
  (params (Interractor :type Character%20Object%20Reference))
  (bind _asbp_first_person_shooter_character (Utilities|Casting|CastToBP_FirstPersonShooterCharacter Interractor))
  ;[0.15 0.15 0.15 0.5] Only pick up if ammo is not full
  (bind _isfull (Default|IsFull (Variables|/Game/Production/Blueprints/BP_FirstPersonShooterCharacter.BP_FirstPersonShooterCharacter_C|GetBPC_AmmoInventory _asbp_first_person_shooter_character) (Variables|Default|GetAmmoType)))
  (if (not _isfull)
    (Default|AddAmmo (Variables|/Game/Production/Blueprints/BP_FirstPersonShooterCharacter.BP_FirstPersonShooterCharacter_C|GetBPC_AmmoInventory _asbp_first_person_shooter_character) (Variables|Default|GetAmmoValue) (Variables|Default|GetAmmoType))
    (Default|CallPickedUp)
    (Actor|DestroyActor)
    (return false)))