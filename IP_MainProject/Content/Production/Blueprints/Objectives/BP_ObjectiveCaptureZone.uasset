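; Objective capture zone that the first-person shooter character completes by staying inside its mesh for an instance-editable capture time.
; First overlap creates a progress widget and starts a timer, leaving pauses it and removes the widget, and re-entry resumes both.
; When the timer expires, it fires the Completed dispatcher, clears the timer and removes the widget.
; Overlaps are ignored while the zone is hidden.
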(event OnComponentBeginOverlap(StaticMesh)
  (params (OverlappedComponent :type Primitive%20Component%20Object%20Reference) (OtherActor :type Actor%20Object%20Reference) (OtherComp :type Primitive%20Component%20Object%20Reference) (OtherBodyIndex :type Integer) (bFromSweep :type Boolean) (SweepResult :type Hit%20Result%20Structure%20%28by%20ref%29))
  (Utilities|Casting|CastToBP_FirstPersonShooterCharacter OtherActor)
  (if (not (Variables|Default|GetbHidden))
    (if (Utilities|Time|IsValidTimerHandle (Variables|Default|GetTimer))
      ;[0.15 0.15 0.15 0.5] If there is already a Timer, unpause it and add ProgressBar to Viewport
      (Utilities|Time|UnpauseTimerbyHandle (Variables|Default|GetTimer))
      (UserInterface|Viewport|AddtoViewport (Variables|Default|GetProgressBar) 0)
      (else
        ;[0.15 0.15 0.15 0.5] Create and add Progress bar to Viewport
        (bind _returnvalue (UserInterface|CreateWidget "/Game/Production/Blueprints/Objectives/UI/WBP_CaptureProgress.WBP_CaptureProgress_C"))
        (bind _output_get (Variables|Default|SetProgressBar _returnvalue))
        (UserInterface|Viewport|AddtoViewport _output_get 0)
        ;[0.15 0.15 0.15 0.5] Set duration of the Timer, CaptureTime is instance editable
        (bind _output_get_2 (Variables|/Game/Production/Blueprints/Objectives/UI/WBP_CaptureProgress.WBP_CaptureProgress_C|SetMaxProgress (Variables|Default|GetProgressBar) (Variables|Default|GetCaptureTime)))
        (bind _returnvalue_2 (Utilities|Time|SetTimerbyEvent (delegate Custom|Captured) _output_get_2))
        (Variables|Default|SetTimer _returnvalue_2)))))

(event OnComponentEndOverlap(StaticMesh)
  (params (OverlappedComponent :type Primitive%20Component%20Object%20Reference) (OtherActor :type Actor%20Object%20Reference) (OtherComp :type Primitive%20Component%20Object%20Reference) (OtherBodyIndex :type Integer))
  (Utilities|Casting|CastToBP_FirstPersonShooterCharacter OtherActor)
  (if (not (Variables|Default|GetbHidden))
    ;[0.15 0.15 0.15 0.5] Pause Timer and Remove from screen
    (Utilities|Time|PauseTimerbyHandle (Variables|Default|GetTimer))
    (Widget|RemovefromParent (Variables|Default|GetProgressBar))))

(event Custom|Captured
  ;[0.15 0.15 0.15 0.5] Once Timer is up, call completed Event Dispatcher and delete Timer and remove Progress bar
  (Default|CallCompleted)
  (Utilities|Time|ClearandInvalidateTimerbyHandle (Variables|Default|GetTimer))
  (Widget|RemovefromParent (Variables|Default|GetProgressBar)))

(fn ConstructionScript
  (|CallParentFunction))