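; BP_ObjectiveManager steps the player through an ordered array of objective actors, showing one at a time.
; On BeginPlay it creates the objective text widget, hides every objective, then activates the current one.
; SetCurrentObjective unhides the actor, displays its instructions and binds to its completion event.
; On completion it re-hides any surviving actor for reuse and advances the index, calling itself when the next entry is invalid.
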(event Custom|OnEventCompleted
  (bind _currentobjectiveindex (Variables|Default|GetCurrentObjectiveIndex))
  (bind _orderedobjectives (Variables|Default|GetOrderedObjectives))
  (bind _output (Utilities|Array|Get(acopy) _orderedobjectives _currentobjectiveindex))
  ;[0.15 0.15 0.15 0.5] If I want to reuse objectives, instead of destorying actor in their bp I set them hidden again if they still exist
  (Utilities|IsValid _output
    (:Is%20Valid
      (Rendering|SetActorHiddenInGame _output true)
      ;[0.15 0.15 0.15 0.5] Set the next element of the Objective array to visible
      (bind _result (Math|Integer|IncrementInt (Variables|Default|GetCurrentObjectiveIndex))
        (:%20%20
          (Utilities|IsValid (Utilities|Array|Get(acopy) (Variables|Default|GetOrderedObjectives) _result)
            (:Is%20Valid
              (CallFunction|SetCurrentObjective (Utilities|Array|Get(acopy) (Variables|Default|GetOrderedObjectives) _result)))
            (:Is%20Not%20Valid
              ;[0.15 0.15 0.15 0.5] If we encounter an invalid Objective, skip it
              (if (< (Math|Integer|Min(Integer) (Variables|Default|GetCurrentObjectiveIndex) 1) (Utilities|Array|Length (Variables|Default|GetOrderedObjectives)))
                (CallFunction|OnEventCompleted)))))))))

(event EventBeginPlay
  ;[0.15 0.15 0.15 0.5] Loop through Objectives array and make them all hidden in  game, then set the first objective in the array as visible
  (if (Utilities|Array|IsNotEmpty (Variables|Default|GetOrderedObjectives))
    (bind _returnvalue (UserInterface|CreateWidget "/Game/Production/Blueprints/Objectives/UI/WBP_ObjectiveText.WBP_ObjectiveText_C"))
    (bind _output_get (Variables|Default|SetObjectiveWidget _returnvalue))
    (UserInterface|Viewport|AddtoViewport _output_get 0)
    (for _array_element (Variables|Default|GetOrderedObjectives)
      (Rendering|SetActorHiddenInGame _array_element true))
    (CallFunction|SetCurrentObjective (Utilities|Array|Get(acopy) (Variables|Default|GetOrderedObjectives) (Variables|Default|GetCurrentObjectiveIndex)))))

(fn ConstructionScript)

(fn SetCurrentObjective
  (params (NewObjective :type BP%20Objective%20Marker%20Base%20Object%20Reference))
  (Rendering|SetActorHiddenInGame NewObjective false)
  (Rendering|Components|TextRender|SetText (Variables|/Game/Production/Blueprints/Objectives/UI/WBP_ObjectiveText.WBP_ObjectiveText_C|GetObjectiveText (Variables|Default|GetObjectiveWidget)) (Utilities|Text|ToText(String) (Variables|/Game/Production/Blueprints/Objectives/BP_ObjectiveMarkerBase.BP_ObjectiveMarkerBase_C|GetInstructions NewObjective)))
  (EventDispatchers|BindEventtoCompleted NewObjective (EventDispatchers|CreateEvent :!event Custom|OnEventCompleted)))