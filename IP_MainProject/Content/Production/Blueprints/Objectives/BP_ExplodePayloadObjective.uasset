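; BP_ExplodePayloadObjective is an objective actor that completes when its referenced Payload explodes.
; On BeginPlay, it checks that the Payload is valid and binds its Finished event to the payload's Exploded dispatcher.
; When that fires, it calls Completed and destroys itself.
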(event Custom|Finished
  (Default|CallCompleted)
  (Actor|DestroyActor))

(event EventBeginPlay
  (bind _payload (Variables|Default|GetPayload))
  (|CallParentFunction)
  (Utilities|IsValid _payload
    (:Is%20Valid
      (EventDispatchers|BindEventtoExploded _payload (delegate Custom|Finished)))))

(event Collision|EventActorBeginOverlap
  (params (OtherActor :type Actor%20Object%20Reference))
  (|CallParentFunction OtherActor) ; This node is disabled and will not be called.\nDrag off pins to build functionality.
)

(fn ConstructionScript
  (|CallParentFunction))