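; BP_ChargeWeaponObjective is an objective actor that completes when its referenced charge station finishes charging.
; On BeginPlay it binds to the station's Charged event, provided the ChargeStation reference is valid.
; When that event fires, it calls Completed and destroys itself.
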(event Custom|Charged
  (Default|CallCompleted)
  (Actor|DestroyActor))

(event EventBeginPlay
  (bind _chargestation (Variables|Default|GetChargeStation))
  (|CallParentFunction)
  (Utilities|IsValid _chargestation
    (:Is%20Valid
      (EventDispatchers|BindEventtoCharged _chargestation (delegate Custom|Charged)))))

(event Collision|EventActorBeginOverlap
  (params (OtherActor :type Actor%20Object%20Reference))
  (|CallParentFunction OtherActor) ; This node is disabled and will not be called.\nDrag off pins to build functionality.
)

(event EventTick
  (params (DeltaSeconds :type Float%20%28single-precision%29))
  (|CallParentFunction DeltaSeconds) ; This node is disabled and will not be called.\nDrag off pins to build functionality.
)

(fn ConstructionScript
  (|CallParentFunction))