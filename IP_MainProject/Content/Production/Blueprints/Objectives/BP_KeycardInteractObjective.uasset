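; Objective actor that completes when its assigned keycard is interacted with.
; On BeginPlay, if the Keycard reference is valid, it binds to that keycard's Interacted event.
; The bound Pickedup handler calls Completed and then destroys the objective actor.
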(event Custom|Pickedup
  (Default|CallCompleted)
  (Actor|DestroyActor))

(event EventBeginPlay
  (bind _keycard (Variables|Default|GetKeycard))
  (|CallParentFunction)
  (Utilities|IsValid _keycard
    (:Is%20Valid
      (EventDispatchers|BindEventtoInteracted _keycard (delegate Custom|Pickedup)))))

(event Collision|EventActorBeginOverlap
  (params (OtherActor :type Actor%20Object%20Reference))
  (|CallParentFunction OtherActor) ; This node is disabled and will not be called.\nDrag off pins to build functionality.
)

(event EventTick
  (params (DeltaSeconds :type Float%20%28single-precision%29))
  (|CallParentFunction DeltaSeconds) ; This node is disabled and will not be called.\nDrag off pins to build functionality.
)

(fn ConstructionScript
  (|CallParentFunction))