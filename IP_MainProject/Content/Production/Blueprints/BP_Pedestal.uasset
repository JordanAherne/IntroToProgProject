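; BP_Pedestal is an interactable, colour-tinted pedestal for placing a collected item as part of a goal unlock.
; Construction applies Colour through a dynamic material, and BeginPlay toggles the visibility of attached BP_PlacedCube actors.
; Interact finds its items among attached actors, printing "collect item" while the BP_Item exists.
; Otherwise it toggles the last attached actor's visibility, stores ItemPlaced from PlacedItem's visibility and runs CheckGoalUnlock.
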(event EventBeginPlay
  (for _array_element (Actor|GetAttachedActors self true false)
    (if (Utilities|ClassIsChildOf (Utilities|GetClass _array_element) "/Game/Production/Blueprints/BP_PlacedCube.BP_PlacedCube_C")
      (Rendering|ToggleVisibility (Variables|/Script/Engine.Actor|GetRootComponent _array_element) true))))

(fn ConstructionScript
  (|CallParentFunction)
  (bind _returnvalue (Rendering|Material|CreateDynamicMaterialInstance (Variables|Default|GetCube) 0 0 "None" :!class /Script/Engine.PrimitiveComponent))
  (Rendering|Material|SetVectorParameterValue _returnvalue "Colour" (Variables|Default|GetColour) :!class /Script/Engine.MaterialInstanceDynamic))

(fn Interact
  (params (Interractor :type Character%20Object%20Reference))
  (for _array_element (Actor|GetAttachedActors self true false)
    (if (Utilities|ClassIsChildOf (Utilities|GetClass _array_element) "/Game/Production/Blueprints/BP_Item.BP_Item_C")
      (LocalVariables|SetItemInLevel _array_element)
      (else
        (bind _output_get (LocalVariables|SetPlacedItem _array_element)))))
  (if (Utilities|IsValid (LocalVariables|GetItemInLevel))
    (Development|PrintString "collect item")
    (else
      (Rendering|ToggleVisibility (Variables|/Script/Engine.Actor|GetRootComponent _array_element) true)
      (Variables|Default|SetItemPlaced (Rendering|IsVisible (Variables|/Script/Engine.Actor|GetRootComponent _output_get)))
      (bind _returnvalue (AddComponent|AddCheckGoalUnlock))
      (Default|CheckGoalUnlock _returnvalue))))