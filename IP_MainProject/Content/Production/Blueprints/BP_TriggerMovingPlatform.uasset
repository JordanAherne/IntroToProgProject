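; BP_TriggerMovingPlatform is a platform that moves when the player enters its trigger box.
; BeginPlay caches the first-person shooter character, and Box overlaps from that actor alone play a timeline.
; The timeline lerps the Cube's relative location from zero to MoveToPoint without sweeping.
; Nothing in the graph reverses or resets the movement.
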(event OnComponentBeginOverlap(Box)
  (params (OverlappedComponent :type Primitive%20Component%20Object%20Reference) (OtherActor :type Actor%20Object%20Reference) (OtherComp :type Primitive%20Component%20Object%20Reference) (OtherBodyIndex :type Integer) (bFromSweep :type Boolean) (SweepResult :type Hit%20Result%20Structure%20%28by%20ref%29))
  (if (== OtherActor (Variables|Default|GetPlayer))
    (bind _movementalpha (Timeline|TL_MovingPlatform Play)
      (:Update
        (Transformation|SetRelativeLocation (Variables|Default|GetCube) (Math|Vector|Lerp(Vector) "0, 0, 0" (Variables|Default|GetMoveToPoint) _movementalpha) false false)))))

(event EventBeginPlay
  (bind _asbp_first_person_shooter_character (Utilities|Casting|CastToBP_FirstPersonShooterCharacter (Game|GetPlayerCharacter 0)))
  (Variables|Default|SetPlayer _asbp_first_person_shooter_character))

(fn ConstructionScript)