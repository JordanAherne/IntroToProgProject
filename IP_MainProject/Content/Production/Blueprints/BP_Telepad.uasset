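; BP_Telepad is a teleport pad that moves an overlapping actor to its Destination after a countdown.
; Begin overlap, unfiltered by actor type, shows a WBP_TeleportCountdown widget and starts a timer using that widget's Countdown value.
; When the timer fires, Teleport prints the destination and moves the actor there with zeroed rotation.
; End overlap clears the timer and removes the widget, so leaving early cancels the teleport.
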(event Custom|Teleport
  (bind _destination (Variables|Default|GetDestination))
  (Development|PrintString (Utilities|String|ToString(Vector) _destination) true true "(R=0.000000,G=0.660000,B=1.000000,A=1.000000)" 22222.0)
  (Transformation|Teleport (stale Collision|EventActorBeginOverlap OtherActor) _destination "0, 0, 0"))

(event Collision|EventActorEndOverlap
  (params (OtherActor :type Actor%20Object%20Reference))
  (Utilities|Time|ClearandInvalidateTimerbyHandle (stale Collision|EventActorBeginOverlap _returnvalue_2))
  (Widget|RemovefromParent (Variables|Default|GetTimerPrompt)))

(event EventBeginPlay)

(event Collision|EventActorBeginOverlap
  (params (OtherActor :type Actor%20Object%20Reference))
  (bind _returnvalue (UserInterface|CreateWidget "/Game/Production/Blueprints/WBP/WBP_TeleportCountdown.WBP_TeleportCountdown_C"))
  (bind _output_get (Variables|Default|SetTimerPrompt _returnvalue))
  (UserInterface|Viewport|AddtoViewport _output_get 0)
  (bind _returnvalue_2 (Utilities|Time|SetTimerbyEvent (delegate Custom|Teleport) (Variables|/Game/Production/Blueprints/WBP/WBP_TeleportCountdown.WBP_TeleportCountdown_C|GetCountdown (Variables|Default|GetTimerPrompt)))))

(fn ConstructionScript)