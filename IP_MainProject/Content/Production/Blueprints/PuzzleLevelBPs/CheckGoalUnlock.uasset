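; CheckGoalUnlock is puzzle level logic that opens or closes the goal door based on whether items are placed on pedestals.
; Its event scans every BP_Pedestal and clears an AllPlaced flag if any lacks a placed item.
; If the flag holds, it hides the BP_GoalDoor cube and disables its collision; otherwise it shows the cube with query and physics collision.
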(event Custom|CheckGoalUnlock
  (bind _outactors (Actor|GetAllActorsOfClass "/Game/Production/Blueprints/PuzzleLevelBPs/BP_Pedestal.BP_Pedestal_C"))
  (for _array_element _outactors
    (if (not (Variables|/Game/Production/Blueprints/PuzzleLevelBPs/BP_Pedestal.BP_Pedestal_C|GetItemPlaced _array_element))
      (Variables|Default|SetallPlaced false)))
  (if (Variables|Default|GetallPlaced)
    (bind _returnvalue (Actor|GetActorOfClass "/Game/Production/Blueprints/PuzzleLevelBPs/BP_GoalDoor.BP_GoalDoor_C"))
    (Rendering|SetVisibility (Variables|/Game/Production/Blueprints/PuzzleLevelBPs/BP_GoalDoor.BP_GoalDoor_C|GetCube _returnvalue) false true)
    (Collision|SetCollisionEnabled (Variables|/Game/Production/Blueprints/PuzzleLevelBPs/BP_GoalDoor.BP_GoalDoor_C|GetCube _returnvalue) "NoCollision")
    (else
      (bind _returnvalue_2 (Actor|GetActorOfClass "/Game/Production/Blueprints/PuzzleLevelBPs/BP_GoalDoor.BP_GoalDoor_C"))
      (Rendering|SetVisibility (Variables|/Game/Production/Blueprints/PuzzleLevelBPs/BP_GoalDoor.BP_GoalDoor_C|GetCube _returnvalue_2) true true)
      (Collision|SetCollisionEnabled (Variables|/Game/Production/Blueprints/PuzzleLevelBPs/BP_GoalDoor.BP_GoalDoor_C|GetCube _returnvalue_2) "QueryAndPhysics"))))