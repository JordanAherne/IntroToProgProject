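; BP_Pedestal is an interactable puzzle pedestal with a tinted cube, used to place a gem.
; On BeginPlay it toggles visibility of attached BP_PlacedItem actors.
; Interact prompts "Collect Gem" while an attached BP_Item is valid; otherwise it toggles the last looped attached actor's visibility.
; It then shows placed or collected text from the placed item's visibility and runs CheckGoalUnlock on a newly added component.
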(event EventBeginPlay
  (for _array_element (Actor|GetAttachedActors self true false)
    (if (Utilities|ClassIsChildOf (Utilities|GetClass _array_element) "/Game/Production/Blueprints/PuzzleLevelBPs/BP_PlacedItem.BP_PlacedItem_C")
      (Rendering|ToggleVisibility (Variables|/Script/Engine.Actor|GetRootComponent _array_element) true))))

(fn ConstructionScript
  (|CallParentFunction)
  (bind _returnvalue (Rendering|Material|CreateDynamicMaterialInstance (Variables|Default|GetCube) 0 0 "None" :!class /Script/Engine.PrimitiveComponent))
  (Rendering|Material|SetVectorParameterValue _returnvalue "DefaultColour" (Variables|Default|GetColour) :!class /Script/Engine.MaterialInstanceDynamic))

(fn Interact
  (params (Interractor :type Character%20Object%20Reference))
  (bind _returnvalue (UserInterface|CreateWidget "/Game/Production/Blueprints/WBP/WBP_Text.WBP_Text_C"))
  (Variables|Default|SetText _returnvalue)
  (for _array_element (Actor|GetAttachedActors self true false)
    ;[0.15 0.15 0.15 0.5] Find Correlated BP_Item and see whether or not it is in the level
    (if (Utilities|ClassIsChildOf (Utilities|GetClass _array_element) "/Game/Production/Blueprints/PuzzleLevelBPs/BP_Item.BP_Item_C")
      (LocalVariables|SetItemInLevel _array_element)
      (else
        (bind _output_get (LocalVariables|SetPlacedItem _array_element)))))
  (if (Utilities|IsValid (LocalVariables|GetItemInLevel))
    (Rendering|Components|TextRender|SetText (Variables|/Game/Production/Blueprints/WBP/WBP_Text.WBP_Text_C|GetTextBlock (Variables|Default|GetText)) "Collect Gem")
    (UserInterface|Viewport|AddtoViewport (Variables|Default|GetText) 0)
    (else
      (Rendering|ToggleVisibility (Variables|/Script/Engine.Actor|GetRootComponent _array_element) true)
      (bind _output_get_2 (Variables|Default|SetItemPlaced (Rendering|IsVisible (Variables|/Script/Engine.Actor|GetRootComponent _output_get))))
      (if _output_get_2
        (Rendering|Components|TextRender|SetText (Variables|/Game/Production/Blueprints/WBP/WBP_Text.WBP_Text_C|GetTextBlock (Variables|Default|GetText)) " Gem Placed")
        (UserInterface|Viewport|AddtoViewport (Variables|Default|GetText) 0)
        (else
          (Rendering|Components|TextRender|SetText (Variables|/Game/Production/Blueprints/WBP/WBP_Text.WBP_Text_C|GetTextBlock (Variables|Default|GetText)) " Gem Collected")
          (UserInterface|Viewport|AddtoViewport (Variables|Default|GetText) 0)))
      (bind _returnvalue_2 (AddComponent|AddCheckGoalUnlock))
      (Default|CheckGoalUnlock _returnvalue_2))))