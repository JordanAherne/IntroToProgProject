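; BP_Item is a collectible gem pickup for the first-person shooter character.
; When that character overlaps its Box, it creates a WBP_Text widget reading "Gem Collected", adds it to the viewport and destroys itself.
; The construction script creates a dynamic material instance on the Cube mesh and applies the Colour variable, so each instance can have its own tint.
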(event OnComponentBeginOverlap(Box)
  (params (OverlappedComponent :type Primitive%20Component%20Object%20Reference) (OtherActor :type Actor%20Object%20Reference) (OtherComp :type Primitive%20Component%20Object%20Reference) (OtherBodyIndex :type Integer) (bFromSweep :type Boolean) (SweepResult :type Hit%20Result%20Structure%20%28by%20ref%29))
  (Utilities|Casting|CastToBP_FirstPersonShooterCharacter OtherActor)
  (bind _returnvalue (UserInterface|CreateWidget "/Game/Production/Blueprints/WBP/WBP_Text.WBP_Text_C"))
  (Variables|Default|SetText _returnvalue)
  (Rendering|Components|TextRender|SetText (Variables|/Game/Production/Blueprints/WBP/WBP_Text.WBP_Text_C|GetTextBlock (Variables|Default|GetText)) " Gem Collected")
  (UserInterface|Viewport|AddtoViewport (Variables|Default|GetText) 0)
  (Actor|DestroyActor))

(fn ConstructionScript
  (|CallParentFunction)
  (bind _returnvalue (Rendering|Material|CreateDynamicMaterialInstance (Variables|Default|GetCube) 0 0 "None" :!class /Script/Engine.PrimitiveComponent))
  (Rendering|Material|SetVectorParameterValue _returnvalue "DefaultColour" (Variables|Default|GetColour) :!class /Script/Engine.MaterialInstanceDynamic))