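; Test interactable actor that shows an interaction prompt when the player character is nearby.
; BeginPlay creates a P_Interact widget, which the Box overlap events add to the viewport when the player character enters and remove when it leaves.
; Its BeginInteraction override calls the parent implementation, then prints a debug message.
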(event OnComponentBeginOverlap(Box)
  (params (OverlappedComponent :type Primitive%20Component%20Object%20Reference) (OtherActor :type Actor%20Object%20Reference) (OtherComp :type Primitive%20Component%20Object%20Reference) (OtherBodyIndex :type Integer) (bFromSweep :type Boolean) (SweepResult :type Hit%20Result%20Structure%20%28by%20ref%29))
  (if (== OtherActor (Game|GetPlayerCharacter 0))
    (UserInterface|Viewport|AddtoViewport (Variables|Default|GetInteractPrompt) 0)))

(event OnComponentEndOverlap(Box)
  (params (OverlappedComponent :type Primitive%20Component%20Object%20Reference) (OtherActor :type Actor%20Object%20Reference) (OtherComp :type Primitive%20Component%20Object%20Reference) (OtherBodyIndex :type Integer))
  (if (== (Game|GetPlayerCharacter 0) OtherActor)
    (Widget|RemovefromParent (Variables|Default|GetInteractPrompt))))

(event EventBeginInteraction
  (|CallParentFunction)
  (Development|PrintString "Interacted"))

(event EventBeginPlay
  (bind _returnvalue (UserInterface|CreateWidget "/Game/Production/Blueprints/P_Interact.P_Interact_C"))
  (Variables|Default|SetInteractPrompt _returnvalue))

(fn ConstructionScript
  (|CallParentFunction))