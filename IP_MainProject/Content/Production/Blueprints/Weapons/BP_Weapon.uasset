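; Weapon Blueprint that fires hitscan shots, with ammo, fire delay and timed reloading.
; Shoot runs one randomly spread line trace per pellet, applying bullet damage scaled by the hit physical material's modifier and pushing simulating components with an impulse.
; Timers gate CanShoot between shots and refill ammo after Reload.
; Debug traces and prints remain, and Interact is only a placeholder print.
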(event Custom|ShootTimerExpired
  (Variables|Default|SetcanShoot true))

(event Custom|ReloadTimerExpired
  (Variables|Default|SetcanShoot true)
  (Variables|Default|SetReloading false)
  (Variables|Default|SetWeaponAmmo (Variables|Default|GetMaxWeaponAmmo)))

(event EventBeginPlay)

(event Collision|EventActorBeginOverlap
  (params (OtherActor :type Actor%20Object%20Reference)))

(event EventTick
  (params (DeltaSeconds :type Float%20%28single-precision%29)))

(fn ConstructionScript)

(fn Shoot
  (params (OriginLocation :type Vector) (ForwardVector :type Vector))
  (bind _bulletspread (Variables|Default|GetBulletSpread))
  (bind _bulletspread_2 (Variables|Default|GetBulletSpread))
  (bind _bulletspread_3 (Variables|Default|GetBulletSpread))
  (if (Math|Boolean|ANDBoolean (> (Variables|Default|GetWeaponAmmo) 0) (Variables|Default|GetcanShoot) (not (Variables|Default|GetReloading)))
    (Variables|Default|SetcanShoot false)
    (Utilities|Time|SetTimerbyEvent (EventDispatchers|CreateEvent :!event Custom|ShootTimerExpired) (Variables|Default|GetFireDelay))
    (Math|Integer|DecrementInt (Variables|Default|GetWeaponAmmo)
      (:%20%20
        ;[0.15 0.15 0.15 0.5] Repeat line trace for multiple pellets
        (for _index (range 0 (- (Variables|Default|GetPelletCount) 1))
          (bind _outhit (Collision|LineTraceByChannel OriginLocation (+ OriginLocation (+ (* ForwardVector (Variables|Default|GetRange)) (Math|Vector|MakeVector (Math|Random|RandomFloatinRange (* _bulletspread_2 -1.0) _bulletspread_2) (Math|Random|RandomFloatinRange (* _bulletspread_3 -1.0) _bulletspread_3) (Math|Random|RandomFloatinRange (* _bulletspread -1.0) _bulletspread)))) "TraceTypeQuery1" false 0 "ForDuration" true "(R=1.000000,G=0.000000,B=0.000000,A=1.000000)" "(R=0.000000,G=1.000000,B=0.000000,A=1.000000)" 1.0))
          (Utilities|IsValid (.hitcomponent _outhit)
            (:Is%20Valid
              (Game|Damage|ApplyDamage (.hitactor _outhit) (* (Variables|Default|GetDamage) (.damagethresholdmultiplier (Variables|/Script/PhysicsCore.PhysicalMaterial|GetDamageModifier (.physmat _outhit)))) (Game|GetPlayerController 0) self "/Engine/EngineDamageTypes/DmgTypeBP_BulletDamage.DmgTypeBP_BulletDamage_C")
              (Development|PrintString (Utilities|String|ToString(Float) (* (Variables|Default|GetDamage) (.damagethresholdmultiplier (Variables|/Script/PhysicsCore.PhysicalMaterial|GetDamageModifier (.physmat _outhit))))))
              (if (Physics|IsSimulatingPhysics (.hitcomponent _outhit) (.bonename _outhit))
                (Physics|AddImpulseatLocation (.hitcomponent _outhit) (* (* (.impactnormal _outhit) -1.0) (Variables|Default|GetImpactForce)) (.impactpoint _outhit) (.hitbonename _outhit))
                (Development|PrintString (Utilities|String|Append "TARGET" (Utilities|GetDisplayName (.hitcomponent _outhit)) "FORCE" (Utilities|String|ToString(Vector) (* (* (.impactnormal _outhit) -1.0) (Variables|Default|GetImpactForce))) "LOCATION" (Utilities|String|ToString(Vector) (.impactpoint _outhit)) "BONE" (Utilities|String|ToString(Name) (.hitbonename _outhit))) true true "(R=0.000000,G=0.660000,B=1.000000,A=1.000000)" 1e+01)))))))))

(fn Reload
  (if (and (< (Variables|Default|GetWeaponAmmo) (Variables|Default|GetMaxWeaponAmmo)) (not (Variables|Default|GetReloading)))
    (Variables|Default|SetcanShoot false)
    (Variables|Default|SetReloading true)
    (Utilities|Time|SetTimerbyEvent (EventDispatchers|CreateEvent :!event Custom|ReloadTimerExpired) (Variables|Default|GetReloadTime))
    (return true)))

(fn StopShooting
  (Variables|Default|SetcanShoot false))

(fn Interact
  (params (Interractor :type Character%20Object%20Reference))
  (Development|PrintString "Hello")
  (return false))