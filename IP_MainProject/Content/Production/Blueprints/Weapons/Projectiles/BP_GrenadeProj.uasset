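; BP_GrenadeProj is a grenade projectile that explodes when it hits something.
; On Hit it strips any active BPC_Shield from the struck actor, then applies full radial damage at the impact point.
; A radial impulse call follows, but its target component is set to None.
; It hides the orb and spawns BP_Explosion, which a timeline scales up before destroying both actors.
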(event Collision|EventHit
  (params (MyComp :type Primitive%20Component%20Object%20Reference) (Other :type Actor%20Object%20Reference) (OtherComp :type Primitive%20Component%20Object%20Reference) (bSelfMoved :type Boolean) (HitLocation :type Vector :default "0, 0, 0") (HitNormal :type Vector :default "0, 0, 0") (NormalImpulse :type Vector :default "0, 0, 0") (Hit :type Hit%20Result%20Structure%20%28by%20ref%29))
  (bind _returnvalue (Actor|GetComponentbyClass Other "/Game/Production/Blueprints/Components/BPC_Shield.BPC_Shield_C"))
  (Variables|Default|SetHit%20Location HitLocation)
  (Variables|Default|SetOther%20Comp 0)
  (Utilities|IsValid _returnvalue
    (:Is%20Valid
      (if (Variables|/Game/Production/Blueprints/Components/BPC_Shield.BPC_Shield_C|GethasShield _returnvalue)
        (Default|RemoveShield _returnvalue)))
    (:Is%20Not%20Valid
      _))
  (Game|Damage|ApplyRadialDamage 5.0 (Variables|Default|GetHit%20Location) 2e+02 0 0 0 0 true "ECC_Visibility")
  (Class|PhysicsObjectBlueprintLibrary|ApplyRadialImpulse (Variables|Default|GetOther%20Comp) (Variables|Default|GetHit%20Location) 5e+03 3e+04 "RIF_Constant" false 0.0 false 1e+03 3e+04)
  (bind _returnvalue_2 (Game|SpawnActorfromClass "/Game/Production/Blueprints/LevelComponents/BP_Explosion.BP_Explosion_C" (Math|Transform|MakeTransform (Variables|Default|GetHit%20Location) "0, 0, 0" "1.000000,1.000000,1.000000") "Undefined" "MultiplyWithRoot" 0 0))
  (Rendering|SetVisibility (Variables|Default|GetOrb) false false)
  (bind _newtrack_0 (Timeline|Timeline Play)
    (:Update
      (Transformation|SetWorldTransform (Variables|/Script/Engine.Actor|GetRootComponent _returnvalue_2) (Math|Transform|MakeTransform (Variables|Default|GetHit%20Location) "0, 0, 0" (Math|Conversions|ToVector(Float) (Math|Float|Lerp 0.0 4.0 _newtrack_0))) false false))
    (:Finished
      (Actor|DestroyActor _returnvalue_2)
      (Actor|DestroyActor))))

(fn ConstructionScript)