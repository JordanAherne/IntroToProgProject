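; BP_Boss is a boss enemy that stays invulnerable until its shield is down and both of its arms are dead.
; PawnSensing detects the first-person player and, while the boss is alive, passes them to TargetPlayer with the Eye component and actor rotation.
; SetArms stores the two arm references and binds to their health death events, with left and right dead flags gating damage to BPCHealth.
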(event OnSeePawn(PawnSensing)
  (params (Pawn :type Pawn%20Object%20Reference))
  (if (not (Variables|/Game/Production/Blueprints/Components/BPC_Health.BPC_Health_C|GetDead (Variables|Default|GetBPC_Health)))
    (bind _asbp_first_person_shooter_character (Utilities|Casting|CastToBP_FirstPersonShooterCharacter Pawn))
    (Variables|Default|SetPlayer _asbp_first_person_shooter_character)
    (CallFunction|TargetPlayer (Variables|Default|GetPlayer) (Variables|Default|GetEye) true)))

(event Custom|SetRightDead
  (Variables|Default|SetRightDead true))

(event Custom|SetLeftDead
  (Variables|Default|SetLeftDead true))

(event EventBeginPlay
  (|CallParentFunction))

(event Game|Damage|EventAnyDamage
  (params (Damage :type Float%20%28single-precision%29) (DamageType :type Damage%20Type%20Object%20Reference) (InstigatedBy :type Controller%20Object%20Reference) (DamageCauser :type Actor%20Object%20Reference))
  (if (Math|Boolean|ANDBoolean (not (Variables|/Game/Production/Blueprints/Components/BPC_Shield.BPC_Shield_C|GethasShield (Variables|Default|GetBPC_Shield))) (Variables|Default|GetLeftDead) (Variables|Default|GetRightDead))
    (Default|HealthUpdate (Variables|Default|GetBPC_Health) Damage)))

(fn ConstructionScript
  (|CallParentFunction))

(fn SetArms
  (params (Left :type BP%20Boss%20Arm%20Object%20Reference) (Right :type BP%20Boss%20Arm%20Object%20Reference))
  (bind _output_get (Variables|Default|SetLeftArm Left))
  (EventDispatchers|BindEventtoOnDeath (Variables|/Game/Production/Blueprints/Enemies/BP_RobotBase.BP_RobotBase_C|GetBPC_Health _output_get) (EventDispatchers|CreateEvent :!event Custom|SetLeftDead))
  (bind _output_get_2 (Variables|Default|SetRightArm Right))
  (EventDispatchers|BindEventtoOnDeath (Variables|/Game/Production/Blueprints/Enemies/BP_RobotBase.BP_RobotBase_C|GetBPC_Health _output_get_2) (EventDispatchers|CreateEvent :!event Custom|SetRightDead)))