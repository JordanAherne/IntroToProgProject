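; Dual-wielding robot enemy that chases the player on sight and fires from alternating left and right arms.
; Pawn sensing, while the robot is active and alive, turns it toward the player and starts an AI move into range.
; On arrival, one BP_TurretGun child actor shoots from the current arm's shoot point, switching arms after each successful shot.
; A five-second timer, cleared on each sighting, returns it to line patrol.
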(event OnSeePawn(PawnSensing)
  (params (Pawn :type Pawn%20Object%20Reference))
  (bind _shootpointl (Variables|Default|GetShootPointL))
  (bind _shootpointr (Variables|Default|GetShootPointR))
  (if (and (not (Variables|/Game/Production/Blueprints/Components/BPC_Health.BPC_Health_C|GetDead (Variables|Default|GetBPC_Health))) (Variables|Default|GetisActive))
    (bind _asbp_first_person_shooter_character (Utilities|Casting|CastToBP_FirstPersonShooterCharacter Pawn))
    (Variables|Default|SetPlayer _asbp_first_person_shooter_character)
    (Variables|Default|SetisSensingPlayer true)
    (Utilities|Time|ClearandInvalidateTimerbyHandle (Variables|Default|GetTimer))
    (CallFunction|TargetPlayer (Variables|Default|GetPlayer) (Variables|Default|GetBody) true)
    (AI|AIMoveTo self "0, 0, 0" (Variables|Default|GetPlayer) (Variables|Default|GetDistance%20to%20player) false
      (:then
        (bind _returnvalue (Utilities|Time|SetTimerbyEvent (delegate Custom|RestartPatrol) 5.0))
        (Variables|Default|SetTimer _returnvalue))
      (:OnSuccess
        (if (Variables|Default|GetShot)
          (CallFunction|TargetPlayer (Variables|Default|GetPlayer) (Variables|Default|GetArmL) true)
          (bind _shot (Default|Shoot (Variables|Default|GetGunBP) (Transformation|GetWorldLocation _shootpointl) (Math|Vector|GetForwardVector _shootpointl)))
          (if _shot
            (Variables|Default|SetShot false))
          (else
            (CallFunction|TargetPlayer (Variables|Default|GetPlayer) (Variables|Default|GetArmR) true)
            (bind _shot_2 (Default|Shoot (Variables|Default|GetGunBP) (Transformation|GetWorldLocation _shootpointr) (Math|Vector|GetForwardVector _shootpointr)))
            (Variables|Default|SetShot _shot_2)))))))

(event Custom|RestartPatrol
  (Variables|Default|SetisSensingPlayer false)
  (CallFunction|LinePatrol))

(event Custom|Inactive
  (|CallParentFunction))

(event Custom|Active
  (|CallParentFunction))

(event EventBeginPlay
  (|CallParentFunction)
  (bind _asbp_turret_gun (Utilities|Casting|CastToBP_TurretGun (Variables|/Script/Engine.ChildActorComponent|GetChildActor (Variables|Default|GetGun))))
  (Variables|Default|SetGunBP _asbp_turret_gun))

(event Collision|EventActorBeginOverlap
  (params (OtherActor :type Actor%20Object%20Reference))
  (|CallParentFunction OtherActor) ; This node is disabled and will not be called.\nDrag off pins to build functionality.
)

(event EventTick
  (params (DeltaSeconds :type Float%20%28single-precision%29))
  (|CallParentFunction DeltaSeconds) ; This node is disabled and will not be called.\nDrag off pins to build functionality.
)

(fn ConstructionScript
  (|CallParentFunction))