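; Enemy that shoots at the first-person player character when it sees them.
; On BeginPlay it spawns a BP_Rifle, attaches it to its GunPivot and fires it along the rifle's forward vector whenever PawnSensing detects the player.
; Incoming damage feeds its health component, whose OnDeath event destroys the enemy.
; No movement logic appears in these graphs, and TargetPlayer is an empty, unused stub.
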(event OnSeePawn(PawnSensing)
  (params (Pawn :type Pawn%20Object%20Reference))
  (bind _weapon (Variables|Default|GetWeapon))
  (Utilities|Casting|CastToBP_FirstPersonShooterCharacter Pawn)
  (Default|Shoot _weapon (Transformation|GetWorldLocation (Variables|/Script/Engine.Actor|GetRootComponent _weapon)) (Math|Vector|GetForwardVector (Variables|/Script/Engine.Actor|GetRootComponent _weapon))))

(event OnDeath(BPC_Health)
  (Actor|DestroyActor))

(event EventBeginPlay
  (bind _returnvalue (Game|SpawnActorfromClass "/Game/Production/Blueprints/Weapons/BP_Rifle.BP_Rifle_C" (Math|Transform|MakeTransform "0, 0, 0" "0.000000,0.000000,90.000000" "1.000000,1.000000,1.000000") "Undefined" "MultiplyWithRoot" 0 0))
  (bind _output_get (Variables|Default|SetWeapon _returnvalue))
  (Transformation|AttachComponentToComponent _output_get (Variables|Default|GetGunPivot) "None" "SnapToTarget" "SnapToTarget" "KeepRelative" true))

(event Game|Damage|EventAnyDamage
  (params (Damage :type Float%20%28single-precision%29) (DamageType :type Damage%20Type%20Object%20Reference) (InstigatedBy :type Controller%20Object%20Reference) (DamageCauser :type Actor%20Object%20Reference))
  ;[0.15 0.15 0.15 0.5] Update Health when taking Damage
  (Default|HealthUpdate (Variables|Default|GetBPC_Health) Damage))

(fn ConstructionScript
  (|CallParentFunction))

(fn TargetPlayer
  (params (Player :type Actor%20Object%20Reference)))