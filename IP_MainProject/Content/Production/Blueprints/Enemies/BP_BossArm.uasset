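; BP_BossArm is an enemy boss arm that aims at the player and fires a turret gun.
; On BeginPlay it caches the BP_BossTurretGun from its Gun child actor.
; When PawnSensing sees the player while the arm is alive, active and its Delay flag is set, it aims, then shoots from ShootPoint.
; Aiming uses interpolated look-at rotation, splitting pitch onto the Arm component and yaw onto the whole actor.
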(event OnSeePawn(PawnSensing)
  (params (Pawn :type Pawn%20Object%20Reference))
  (bind _shootpoint (Variables|Default|GetShootPoint))
  (if (Math|Boolean|ANDBoolean (not (Variables|/Game/Production/Blueprints/Components/BPC_Health.BPC_Health_C|GetDead (Variables|Default|GetBPC_Health))) (Variables|Default|GetisActive) (Variables|Default|GetDelay))
    (bind _asbp_first_person_shooter_character (Utilities|Casting|CastToBP_FirstPersonShooterCharacter Pawn))
    (Variables|Default|SetPlayer _asbp_first_person_shooter_character)
    (CallFunction|TargetPlayer (Variables|Default|GetPlayer) (Variables|Default|GetArm) false)
    (Default|Shoot (Variables|Default|GetAs%20BP%20Boss%20Turret%20Gun) (Transformation|GetWorldLocation _shootpoint) (Math|Vector|GetForwardVector _shootpoint))))

(event Collision|EventActorBeginOverlap
  (params (OtherActor :type Actor%20Object%20Reference)))

(event EventTick
  (params (DeltaSeconds :type Float%20%28single-precision%29)))

(event EventBeginPlay
  (|CallParentFunction)
  (bind _asbp_boss_turret_gun (Utilities|Casting|CastToBP_BossTurretGun (Variables|/Script/Engine.ChildActorComponent|GetChildActor (Variables|Default|GetGun))))
  (Variables|Default|SetAs%20BP%20Boss%20Turret%20Gun _asbp_boss_turret_gun))

(fn ConstructionScript
  (|CallParentFunction))

(fn TargetPlayer
  (params (Player :type Actor%20Object%20Reference) (Component :type Static%20Mesh%20Component%20Object%20Reference) (ActorRot :type Boolean))
  (bind _returnvalue (Transformation|GetWorldRotation Component))
  (bind _returnvalue_2 (Utilities|Time|GetWorldDeltaSeconds))
  (bind _returnvalue_3 (Transformation|GetWorldLocation Component))
  (bind _returnvalue_4 (Transformation|GetActorLocation Player))
  (bind _rotationspeed (Variables|Default|GetRotationSpeed))
  (bind _returnvalue_5 (Math|Rotator|FindLookatRotation _returnvalue_3 _returnvalue_4))
  (bind _returnvalue_6 (Math|Interpolation|RInterpTo _returnvalue _returnvalue_5 _returnvalue_2 _rotationspeed))
  (Transformation|SetRelativeRotation Component (Math|Rotator|MakeRotator 0.0 (- (.pitch _returnvalue_6) 1.0) 0.0) false false)
  (Transformation|SetActorRotation (Math|Rotator|MakeRotator 0.0 0.0 (.yaw _returnvalue_6))))