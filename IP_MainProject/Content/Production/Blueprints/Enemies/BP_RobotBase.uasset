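; Base Blueprint for robot enemies, providing damage handling and player aiming.
; AnyDamage forwards incoming damage to the BPCHealth component's HealthUpdate.
; TargetPlayer smoothly interpolates toward the player at RotationSpeed, splitting the aim between clamped pitch on a supplied component and yaw on the whole actor.
; BeginPlay and Tick are empty, so nothing in this Blueprint calls TargetPlayer.
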(event EventBeginPlay)

(event Collision|EventActorBeginOverlap
  (params (OtherActor :type Actor%20Object%20Reference)))

(event EventTick
  (params (DeltaSeconds :type Float%20%28single-precision%29)))

(event Game|Damage|EventAnyDamage
  (params (Damage :type Float%20%28single-precision%29) (DamageType :type Damage%20Type%20Object%20Reference) (InstigatedBy :type Controller%20Object%20Reference) (DamageCauser :type Actor%20Object%20Reference))
  (Default|HealthUpdate (Variables|Default|GetBPC_Health) Damage))

(fn ConstructionScript)

(fn TargetPlayer
  (params (Player :type Actor%20Object%20Reference) (Component :type Static%20Mesh%20Component%20Object%20Reference))
  (bind _returnvalue (Transformation|GetWorldRotation Component))
  (bind _returnvalue_2 (Utilities|Time|GetWorldDeltaSeconds))
  (bind _returnvalue_3 (Transformation|GetWorldLocation Component))
  (bind _returnvalue_4 (Transformation|GetActorLocation Player))
  (bind _rotationspeed (Variables|Default|GetRotationSpeed))
  (bind _returnvalue_5 (Math|Rotator|FindLookatRotation _returnvalue_3 _returnvalue_4))
  (bind _returnvalue_6 (Math|Interpolation|RInterpTo _returnvalue _returnvalue_5 _returnvalue_2 _rotationspeed))
  (Transformation|SetRelativeRotation Component (Math|Rotator|MakeRotator 0.0 (Math|Float|Clamp(Float) (.pitch _returnvalue_6) -2e+01 2e+01) 0.0) false false)
  (Transformation|SetActorRotation (Math|Rotator|MakeRotator 0.0 0.0 (.yaw _returnvalue_6))))