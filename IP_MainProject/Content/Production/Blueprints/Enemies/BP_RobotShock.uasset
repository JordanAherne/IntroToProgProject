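; BP_RobotShock is an enemy robot that chases a seen first-person player and, on reaching them, deals damage and pauses.
; PawnSensing triggers AI MoveTo and player targeting; a successful hit turns the eye blue and starts a timer that re-arms the robot.
; Death or starting inactive drops the body into physics and hides the float beam.
; An Active event restores both, easing the body toward its stored start transform.
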(event OnDeath(BPC_Health)
  (CallFunction|Inactive))

(event OnSeePawn(PawnSensing)
  (params (Pawn :type Pawn%20Object%20Reference))
  (if (and (not (Variables|/Game/Production/Blueprints/Components/BPC_Health.BPC_Health_C|GetDead (Variables|Default|GetBPC_Health))) (Variables|Default|GetisActive))
    (bind _asbp_first_person_shooter_character (Utilities|Casting|CastToBP_FirstPersonShooterCharacter Pawn))
    (Variables|Default|SetPlayer _asbp_first_person_shooter_character)
    (AI|AIMoveTo self "0, 0, 0" (Variables|Default|GetPlayer) (Variables|Default|GetDistance%20to%20player) false
      (:then
        (CallFunction|TargetPlayer (Variables|Default|GetPlayer) (Variables|Default|GetBody)))
      (:OnSuccess
        (Rendering|Material|SetMaterial (Variables|Default|GetEye) 0 "/Game/Production/Materials/M_BlueEmissive.M_BlueEmissive")
        (Game|Damage|ApplyDamage (Variables|Default|GetPlayer) (Variables|Default|GetBase%20Damage) 0 self "/Engine/EngineDamageTypes/DmgTypeBP_Explosive.DmgTypeBP_Explosive_C")
        (Variables|Default|SetisActive false)
        (bind _returnvalue (Utilities|Time|SetTimerbyEvent (delegate Custom|Pause) 5.0))
        (Variables|Default|SetPauseTimer _returnvalue)))))

(event Custom|Pause
  (Variables|Default|SetisActive true)
  (Rendering|Material|SetMaterial (Variables|Default|GetEye) 0 "/Game/Production/Materials/M_CardReaderLocked.M_CardReaderLocked"))

(event Custom|Active
  (bind _starttransformation (Variables|Default|GetStartTransformation))
  (Rendering|Material|SetMaterial (Variables|Default|GetEye) 0 "/Game/Production/Materials/M_CardReaderLocked.M_CardReaderLocked")
  (Rendering|SetVisibility (Variables|Default|GetFloatyBeam) true false)
  (Physics|SetSimulatePhysics (Variables|Default|GetBody) false)
  (Components|MoveComponentTo (Variables|Default|GetBody) (.location _starttransformation) (.rotation _starttransformation) true true 1.0 false)
  (Variables|Default|SetisActive true))

(event Custom|Inactive
  (Variables|Default|SetisActive false)
  (Utilities|Time|ClearandInvalidateTimerbyHandle (Variables|Default|GetPauseTimer))
  (Rendering|Material|SetMaterial (Variables|Default|GetEye) 0 "/Game/Production/Blueprints/PuzzleLevelBPs/NewMaterial.NewMaterial")
  (Rendering|SetVisibility (Variables|Default|GetFloatyBeam) false false)
  (Physics|SetSimulatePhysics (Variables|Default|GetBody) true))

(event EventBeginPlay
  (|CallParentFunction)
  (Variables|Default|SetStartTransformation (Transformation|GetWorldTransform (Variables|Default|GetCapsule)))
  (if (not (Variables|Default|GetisActive))
    (CallFunction|Inactive)))

(event Collision|EventActorBeginOverlap
  (params (OtherActor :type Actor%20Object%20Reference))
  (|CallParentFunction OtherActor) ; This node is disabled and will not be called.\nDrag off pins to build functionality.
)

(event EventTick
  (params (DeltaSeconds :type Float%20%28single-precision%29))
  (|CallParentFunction DeltaSeconds) ; This node is disabled and will not be called.\nDrag off pins to build functionality.
)

(event Game|Damage|EventAnyDamage
  (params (Damage :type Float%20%28single-precision%29) (DamageType :type Damage%20Type%20Object%20Reference) (InstigatedBy :type Controller%20Object%20Reference) (DamageCauser :type Actor%20Object%20Reference))
  (Default|HealthUpdate (Variables|Default|GetBPC_Health) Damage))

(fn ConstructionScript
  (|CallParentFunction))