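; BP_RobotEnemy is an enemy robot that chases the first-person player on sight and shoots with two alternating arms.
; Pawn sensing triggers an AI move; on success, a FlipFlop aims one arm and fires its child-actor turret gun from that side's shoot point.
; Aiming interpolates clamped arm pitch and whole-actor yaw.
; Damage feeds a health component whose death event destroys the robot; an idle head-sweep timeline is unused.
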(event OnDeath(BPC_Health)
  (Actor|DestroyActor))

(event OnSeePawn(PawnSensing)
  (params (Pawn :type Pawn%20Object%20Reference))
  (bind _shootpoint (Variables|Default|GetShootPoint))
  (bind _shootpoint1 (Variables|Default|GetShootPoint1))
  (bind _asbp_first_person_shooter_character (Utilities|Casting|CastToBP_FirstPersonShooterCharacter Pawn))
  (Variables|Default|SetPlayer _asbp_first_person_shooter_character)
  (if (not (Variables|/Game/Production/Blueprints/Components/BPC_Health.BPC_Health_C|GetDead (Variables|Default|GetBPC_Health)))
    (AI|AIMoveTo self (Math|Vector|MakeVector 0.0 0.0 0.0) (Variables|Default|GetPlayer) (Variables|Default|GetDistance%20to%20player) false
      (:OnSuccess
        (Utilities|FlowControl|FlipFlop
          (:A
            (CallFunction|TargetPlayer (Variables|Default|GetPlayer) (Variables|Default|GetHead1))
            (Default|Shoot (Variables|Default|GetGunBP) (Transformation|GetWorldLocation _shootpoint) (Math|Vector|GetForwardVector _shootpoint)))
          (:B
            (CallFunction|TargetPlayer (Variables|Default|GetPlayer) (Variables|Default|GetHead))
            (Default|Shoot (Variables|Default|GetGunBP) (Transformation|GetWorldLocation _shootpoint1) (Math|Vector|GetForwardVector _shootpoint1))))))))

(event EventBeginPlay
  (bind _asbp_turret_gun (Utilities|Casting|CastToBP_TurretGun (Variables|/Script/Engine.ChildActorComponent|GetChildActor (Variables|Default|GetGun))))
  (Variables|Default|SetGunBP _asbp_turret_gun))

(event Game|Damage|EventAnyDamage
  (params (Damage :type Float%20%28single-precision%29) (DamageType :type Damage%20Type%20Object%20Reference) (InstigatedBy :type Controller%20Object%20Reference) (DamageCauser :type Actor%20Object%20Reference))
  (Default|HealthUpdate (Variables|Default|GetBPC_Health) Damage))

(fn ConstructionScript)

(fn TargetPlayer
  (params (Player :type Actor%20Object%20Reference) (Arm :type Static%20Mesh%20Component%20Object%20Reference))
  (bind _returnvalue (Transformation|GetWorldRotation Arm))
  (bind _returnvalue_2 (Utilities|Time|GetWorldDeltaSeconds))
  (bind _returnvalue_3 (Transformation|GetWorldLocation Arm))
  (bind _returnvalue_4 (Transformation|GetActorLocation Player))
  (bind _rotationspeed (Variables|Default|GetRotationSpeed))
  (bind _returnvalue_5 (Math|Rotator|FindLookatRotation _returnvalue_3 _returnvalue_4))
  (bind _returnvalue_6 (Math|Interpolation|RInterpTo _returnvalue _returnvalue_5 _returnvalue_2 _rotationspeed))
  (Transformation|SetRelativeRotation Arm (Math|Rotator|MakeRotator 0.0 (Math|Float|Clamp(Float) (.pitch _returnvalue_6) -2e+01 2e+01) 0.0) false false)
  (Transformation|SetActorRotation (Math|Rotator|MakeRotator 0.0 0.0 (.yaw _returnvalue_6))))