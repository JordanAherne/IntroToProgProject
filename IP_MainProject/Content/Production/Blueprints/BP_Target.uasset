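; BP_Target is a moving target actor that briefly changes colour when it takes any damage.
; The construction script gives the Cube a dynamic material set to the default colour and adds InterpToMovement control points from its origin to a relative Destination.
; On damage it sets the material's DefaultColour parameter to the damaged colour, and a short timer event restores the default.
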(event Custom|ResetColour
  (Rendering|Material|SetVectorParameterValue (Variables|Default|GetMaterial) "DefaultColour" (Variables|Default|GetDefault%20Colour) :!class /Script/Engine.MaterialInstanceDynamic))

(event EventBeginPlay)

(event Collision|EventActorBeginOverlap
  (params (OtherActor :type Actor%20Object%20Reference)))

(event EventTick
  (params (DeltaSeconds :type Float%20%28single-precision%29)))

(event Game|Damage|EventAnyDamage
  (params (Damage :type Float%20%28single-precision%29) (DamageType :type Damage%20Type%20Object%20Reference) (InstigatedBy :type Controller%20Object%20Reference) (DamageCauser :type Actor%20Object%20Reference))
  (Rendering|Material|SetVectorParameterValue (Variables|Default|GetMaterial) "DefaultColour" (Variables|Default|GetDamagedColour) :!class /Script/Engine.MaterialInstanceDynamic)
  (Utilities|Time|SetTimerbyEvent (delegate Custom|ResetColour) 0.3))

(fn ConstructionScript
  (bind _returnvalue (Rendering|Material|CreateDynamicMaterialInstance (Variables|Default|GetCube) 0 0 "None" :!class /Script/Engine.PrimitiveComponent))
  (bind _output_get (Variables|Default|SetMaterial _returnvalue))
  (Rendering|Material|SetVectorParameterValue _output_get "DefaultColour" (Variables|Default|GetDefault%20Colour) :!class /Script/Engine.MaterialInstanceDynamic)
  (Class|InterptoMovementComponent|AddControlPointPosition (Variables|Default|GetInterpToMovement) "0, 0, 0" true)
  (Class|InterptoMovementComponent|AddControlPointPosition (Variables|Default|GetInterpToMovement) (Variables|Default|GetDestination) true))