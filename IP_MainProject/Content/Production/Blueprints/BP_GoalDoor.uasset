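; BP_GoalDoor is a goal door that opens by destroying itself once the level's collectibles are gone.
; Tick polls GetActorOfClass for BP_TestOverlap and BP_TestInteractable, and when neither exists it prints a message and destroys the first BP_GoalDoor found.
; BeginInteraction reuses those lookups to print which items are still needed.
; A box overlap shows and hides the P_Interact prompt widget, created on BeginPlay, for the player.
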(event OnComponentBeginOverlap(Box)
  (params (OverlappedComponent :type Primitive%20Component%20Object%20Reference) (OtherActor :type Actor%20Object%20Reference) (OtherComp :type Primitive%20Component%20Object%20Reference) (OtherBodyIndex :type Integer) (bFromSweep :type Boolean) (SweepResult :type Hit%20Result%20Structure%20%28by%20ref%29))
  ;[0.15 0.15 0.15 0.5] Shows/removes interact prompt
  (if (== OtherActor (Game|GetPlayerCharacter 0))
    (UserInterface|Viewport|AddtoViewport (Variables|Default|GetInteract%20Prompt) 0)))

(event OnComponentEndOverlap(Box)
  (params (OverlappedComponent :type Primitive%20Component%20Object%20Reference) (OtherActor :type Actor%20Object%20Reference) (OtherComp :type Primitive%20Component%20Object%20Reference) (OtherBodyIndex :type Integer))
  ;[0.15 0.15 0.15 0.5] Shows/removes interact prompt
  (if (== (Game|GetPlayerCharacter 0) OtherActor)
    (Widget|RemovefromParent (Variables|Default|GetInteract%20Prompt))))

(event EventBeginPlay
  (bind _returnvalue (UserInterface|CreateWidget "/Game/Production/Blueprints/P_Interact.P_Interact_C"))
  (Variables|Default|SetInteract%20Prompt _returnvalue))

(event EventBeginInteraction
  (if (Utilities|IsValid (stale EventTick _returnvalue_2))
    (if (Utilities|IsValid (stale EventTick _returnvalue))
      (Development|PrintString "Collect \"interactable\" and \"Overlappable\"")
      (else
        (Development|PrintString "Collect \"interactable\"")))
    (else
      (Development|PrintString "Collect \"Overlappable\""))))

(event EventTick
  (params (DeltaSeconds :type Float%20%28single-precision%29))
  (bind _returnvalue (Actor|GetActorOfClass "/Game/Production/Blueprints/BP_TestOverlap.BP_TestOverlap_C"))
  (bind _returnvalue_2 (Actor|GetActorOfClass "/Game/Production/Blueprints/BP_TestInteractable.BP_TestInteractable_C"))
  (if (not (Utilities|IsValid _returnvalue_2))
    (if (not (Utilities|IsValid _returnvalue))
      (Development|PrintString "THE GOAL HAS OPENED")
      (bind _returnvalue_3 (Actor|GetActorOfClass "BP_GoalDoor_C"))
      (Actor|DestroyActor _returnvalue_3))))

(fn ConstructionScript)